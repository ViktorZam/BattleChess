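; Player controller for the online game lobby, handling player names, chat, kicking the client and starting the match via listen-server travel.
; Events loop over the game mode's controller list to relay chat and lobby settings, using network role to target host or client.
; Each side merges incoming info into the game instance's GameInformation, preserving its own identity, then refreshes the HUD's lobby widget.
; The client update also fires a one-shot completion dispatcher.
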(event `self.ReceiveBeginPlay`
  (if (`self.IsLocalPlayerController`)
    (`WidgetBlueprintLibrary.SetInputMode_UIOnlyEx` self (`/Game/Blueprints/LobbyOnlineGame/BP_LobbyOnlineGameHUD.LobbyCreateOnlineGameWidget` (cast `/Game/Blueprints/LobbyOnlineGame/BP_LobbyOnlineGameHUD` (`self.GetHUD`) :!pure true)))))

(event `KickPlayerFromLobby`
  ;[1 1 1] Kick Player
  (for _array_element (`/Game/Blueprints/LobbyOnlineGame/BP_LobbyOnlineGameGM.PlayerController` (cast `/Game/Blueprints/LobbyOnlineGame/BP_LobbyOnlineGameGM` (`GameplayStatics.GetGameMode`) :!pure true))
    (if (`|EnumEquality` (`self.GetRemoteRole` _array_element) "ROLE_AutonomousProxy")
      (`self.GoToMainMenu` _array_element))))

(event `SendMessageOnServer`
  (params (TextMessage :type "Text (by ref)") (`Client/Host` :type Boolean) (SenderPlayerId :type String))
  ;[1 1 1] Sending chat message
  (for _array_element (`/Game/Blueprints/LobbyOnlineGame/BP_LobbyOnlineGameGM.PlayerController` (cast `/Game/Blueprints/LobbyOnlineGame/BP_LobbyOnlineGameGM` (`GameplayStatics.GetGameMode`) :!pure true))
    (if (!= _array_element self)
      (`self.SendMessageToDestination` _array_element TextMessage `Client/Host`))))

(event `SetPlayerName/Id`
  (params (PlayerId :type String) (PlayerName :type String))
  ;[1 1 1] InitPlayersInfo
  (`self.SetPlayerName/Id_Function` PlayerId PlayerName))

(event `GoToMainMenu`
  ;[1 1 1] Kick Player
  (set `/Game/Blueprints/BP_GameInstance.GameInformation` (struct) (`/Game/Blueprints/Library/BP_FunctionLibrary.GetMyGameInstance`))
  (`GameplayStatics.OpenLevelBySoftObjectPtr` "/Game/Maps/L_MainMenu.L_MainMenu"))

(event `SendMessageToDestination`
  (params (TextMessage :type "Text (by ref)") (`Client/Host` :type Boolean))
  ;[1 1 1] Sending chat message
  (`/Game/Widgets/LobbyOnlineGame/WBP_LobbyCreateOnlineGame.WriteMessage` (`/Game/Blueprints/LobbyOnlineGame/BP_LobbyOnlineGameHUD.LobbyCreateOnlineGameWidget` (cast `/Game/Blueprints/LobbyOnlineGame/BP_LobbyOnlineGameHUD` (`self.GetHUD`) :!pure true)) TextMessage `Client/Host`))

(event `StartGame`
  (params (MapNameInEditor :type String))
  (`KismetSystemLibrary.ExecuteConsoleCommand` (`KismetStringLibrary.Concat_StrStr` "servertravel " MapNameInEditor "?listen") null))

(event `SetInfoLobbyOnlineGameForHost`
  (params (GameInfo :type "/Game/Data/UI/Structures/F_GameInformation Structure"))
  (bind (_playernames _gamename _colorfigures _mapname _modifiers _spells _passwordlobby _playerready) (break `/Game/Data/UI/Structures/F_GameInformation` GameInfo))
  (bind _playernames_2 (break `/Game/Data/UI/Structures/F_GameInformation` (`/Game/Blueprints/BP_GameInstance.GameInformation` (`/Game/Blueprints/Library/BP_FunctionLibrary.GetMyGameInstance`))))
  ;[1 1 1] Update Game info for Client/Host
  (if (`|EnumEquality` (`self.GetLocalRole`) "ROLE_Authority")
    (bind _output_get (set `/Game/Blueprints/BP_GameInstance.GameInformation` (make `/Game/Data/UI/Structures/F_GameInformation` (make `/Game/Data/UI/Structures/F_HostClientNamePlayer` (break `/Game/Data/UI/Structures/F_HostClientNamePlayer` _playernames_2) (`.HostPlayerId_9_51E9EE71466647897F50CF820ECE73B7` (break `/Game/Data/UI/Structures/F_HostClientNamePlayer` _playernames_2)) (`.ClientNamePlayer_6_52E95D4541D8224522E6849C0437FB63` (break `/Game/Data/UI/Structures/F_HostClientNamePlayer` _playernames)) (`.ClientPlayerId_11_E24C465647F1969BE6977CB35D6B05A4` (break `/Game/Data/UI/Structures/F_HostClientNamePlayer` _playernames)) (`.SelfName_14_D9DC6BDC4765F733B0CF0D8BF55182D0` (break `/Game/Data/UI/Structures/F_HostClientNamePlayer` _playernames_2))) _gamename _colorfigures _mapname _modifiers _spells _passwordlobby _playerready) (`/Game/Blueprints/Library/BP_FunctionLibrary.GetMyGameInstance`)))
    (`/Game/Widgets/LobbyOnlineGame/WBP_LobbyCreateOnlineGame.SetInfoLobby` (`/Game/Blueprints/LobbyOnlineGame/BP_LobbyOnlineGameHUD.LobbyCreateOnlineGameWidget` (cast `/Game/Blueprints/LobbyOnlineGame/BP_LobbyOnlineGameHUD` (`self.GetHUD`) :!pure true)) _output_get)))

(event `UpdateGameInfoForHost`
  (params (GameInfo :type "/Game/Data/UI/Structures/F_GameInformation Structure"))
  ;[1 1 1] Update Game info for Client/Host
  (for _array_element (`/Game/Blueprints/LobbyOnlineGame/BP_LobbyOnlineGameGM.PlayerController` (cast `/Game/Blueprints/LobbyOnlineGame/BP_LobbyOnlineGameGM` (`GameplayStatics.GetGameMode`) :!pure true))
    (`self.SetInfoLobbyOnlineGameForHost` _array_element GameInfo)))

(event `UpdateGameInfoOnlineLobbyForClient`
  ;[1 1 1] Update Game info for Client/Host
  (for _array_element (`/Game/Blueprints/LobbyOnlineGame/BP_LobbyOnlineGameGM.PlayerController` (cast `/Game/Blueprints/LobbyOnlineGame/BP_LobbyOnlineGameGM` (`GameplayStatics.GetGameMode`) :!pure true))
    (`self.SetInfoLobbyOnlineGameForClient` _array_element (`/Game/Blueprints/BP_GameInstance.GameInformation` (`/Game/Blueprints/Library/BP_FunctionLibrary.GetMyGameInstance`)))))

(event `SetInfoLobbyOnlineGameForClient`
  (params (GameInfo :type "/Game/Data/UI/Structures/F_GameInformation Structure"))
  (bind (_playernames _gamename _colorfigures _mapname _modifiers _spells _passwordlobby _playerready) (break `/Game/Data/UI/Structures/F_GameInformation` GameInfo))
  (bind _playernames_2 (break `/Game/Data/UI/Structures/F_GameInformation` GameInfo))
  (bind _playernames_3 (break `/Game/Data/UI/Structures/F_GameInformation` (`/Game/Blueprints/BP_GameInstance.GameInformation` (`/Game/Blueprints/Library/BP_FunctionLibrary.GetMyGameInstance`))))
  ;[1 1 1] Update Game info for Client/Host
  (`KismetSystemLibrary.PrintString` "Hello")
  (if (`|EnumEquality` (`self.GetLocalRole`) "ROLE_AutonomousProxy")
    (bind _output_get (set `/Game/Blueprints/BP_GameInstance.GameInformation` (make `/Game/Data/UI/Structures/F_GameInformation` (make `/Game/Data/UI/Structures/F_HostClientNamePlayer` (break `/Game/Data/UI/Structures/F_HostClientNamePlayer` _playernames_2) (`.HostPlayerId_9_51E9EE71466647897F50CF820ECE73B7` (break `/Game/Data/UI/Structures/F_HostClientNamePlayer` _playernames_2)) (`.ClientNamePlayer_6_52E95D4541D8224522E6849C0437FB63` (break `/Game/Data/UI/Structures/F_HostClientNamePlayer` _playernames_3)) (`.ClientPlayerId_11_E24C465647F1969BE6977CB35D6B05A4` (break `/Game/Data/UI/Structures/F_HostClientNamePlayer` _playernames_3)) (`.SelfName_14_D9DC6BDC4765F733B0CF0D8BF55182D0` (break `/Game/Data/UI/Structures/F_HostClientNamePlayer` _playernames_3))) _gamename _colorfigures _mapname _modifiers _spells _passwordlobby _playerready) (`/Game/Blueprints/Library/BP_FunctionLibrary.GetMyGameInstance`)))
    (`/Game/Widgets/LobbyOnlineGame/WBP_LobbyCreateOnlineGame.SetInfoLobby` (`/Game/Blueprints/LobbyOnlineGame/BP_LobbyOnlineGameHUD.LobbyCreateOnlineGameWidget` (cast `/Game/Blueprints/LobbyOnlineGame/BP_LobbyOnlineGameHUD` (`self.GetHUD`) :!pure true)) _output_get)
    (`self.CompleteSetInfoLobby`)
    (clear `self.CompleteSetInfoLobby`)))

(fn `SetPlayerName/Id_Function`
  (params (PlayerId :type String) (PlayerName :type String))
  (bind _playername (`local.PlayerName`))
  (bind _playername_2 (`local.PlayerName`))
  (bind _playernames (break `/Game/Data/UI/Structures/F_GameInformation` (`/Game/Blueprints/BP_GameInstance.GameInformation` (`/Game/Blueprints/Library/BP_FunctionLibrary.GetMyGameInstance`))))
  (bind _playernames_2 (break `/Game/Data/UI/Structures/F_GameInformation` (`/Game/Blueprints/BP_GameInstance.GameInformation` (`/Game/Blueprints/Library/BP_FunctionLibrary.GetMyGameInstance`))))
  (if (`|EnumEquality` (`self.GetLocalRole`) "ROLE_Authority")
    (setmembers `/Game/Data/UI/Structures/F_GameInformation` :`StructRef` (`/Game/Blueprints/BP_GameInstance.GameInformation` (`/Game/Blueprints/Library/BP_FunctionLibrary.GetMyGameInstance`)) :`PlayerNames` (make `/Game/Data/UI/Structures/F_HostClientNamePlayer` _playername (`local.PlayerId`) (`.ClientNamePlayer_6_52E95D4541D8224522E6849C0437FB63` (break `/Game/Data/UI/Structures/F_HostClientNamePlayer` _playernames)) (`.ClientPlayerId_11_E24C465647F1969BE6977CB35D6B05A4` (break `/Game/Data/UI/Structures/F_HostClientNamePlayer` _playernames)) _playername))
    (else
      (setmembers `/Game/Data/UI/Structures/F_GameInformation` :`StructRef` (`/Game/Blueprints/BP_GameInstance.GameInformation` (`/Game/Blueprints/Library/BP_FunctionLibrary.GetMyGameInstance`)) :`PlayerNames` (make `/Game/Data/UI/Structures/F_HostClientNamePlayer` (break `/Game/Data/UI/Structures/F_HostClientNamePlayer` _playernames_2) (`.HostPlayerId_9_51E9EE71466647897F50CF820ECE73B7` (break `/Game/Data/UI/Structures/F_HostClientNamePlayer` _playernames_2)) _playername_2 (`local.PlayerId`) _playername_2)))))

(fn `UserConstructionScript`)