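; Game mode for the online lobby that tracks connected lobby player controllers and gives each joining player its identity.
; PostLogin adds the controller to an array and calls SetDataForClientAndHost, while OnLogout removes it.
; That function passes the PlayerState's name and unique net ID string to the controller's SetPlayerNameId, using the same call for AutonomousProxy and SimulatedProxy remote roles to cover client and host.
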(event `self.K2_PostLogin`
  (params (NewPlayer :type "PlayerController Object Reference"))
  (bind _asbp_lobby_online_game_pc (cast `/Game/Blueprints/LobbyOnlineGame/BP_LobbyOnlineGamePC` NewPlayer :!pure true))
  (`KismetArrayLibrary.Array_AddUnique` (`self.PlayerController`) _asbp_lobby_online_game_pc)
  (`self.Set Data for Client and Host` _asbp_lobby_online_game_pc))

(event `self.K2_OnLogout`
  (params (ExitingController :type "Controller Object Reference"))
  (`KismetArrayLibrary.Array_RemoveItem` (`self.PlayerController`) (cast `/Game/Blueprints/LobbyOnlineGame/BP_LobbyOnlineGamePC` ExitingController :!pure true)))

(fn `Set Data for Client and Host`
  (params (PlayerController :type "/Game/Blueprints/LobbyOnlineGame/BP_LobbyOnlineGamePC Object Reference"))
  (bind _playercontroller (`local.PlayerController`))
  (bind _playerstate (`Controller.PlayerState` _playercontroller))
  (if (`|EnumEquality` (`self.GetRemoteRole` (`local.PlayerController`)) "ROLE_AutonomousProxy")
    (`/Game/Blueprints/LobbyOnlineGame/BP_LobbyOnlineGamePC.SetPlayerName/Id` _playercontroller (`AdvancedSessionsLibrary.UniqueNetIdToString` (`AdvancedSessionsLibrary.GetUniqueNetIDFromPlayerState` _playerstate)) (`PlayerState.GetPlayerName` _playerstate) :!label _label)
    (elif (`|EnumEquality` (`self.GetRemoteRole` (`local.PlayerController`)) "ROLE_SimulatedProxy")
      (goto _label))))

(fn `UserConstructionScript`)