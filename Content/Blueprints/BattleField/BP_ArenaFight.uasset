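; BP_ArenaFight stages a scripted arena duel between a white and a black figure, with WhiteWin deciding the outcome.
; Chained montages alternate three attack and hit exchanges, the winner striking first and last, before the loser's death animation plays.
; On authority, a timer shows a "Skip Fight?" prompt shortly after the start.
; The death montage's EndMontage notify hides that prompt and requests the return to the battlefield.
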(event `StartArenaBattle`
  (`/Engine/EditorBlueprintResources/ActorMacros.Switch Has Authority`
    (:`Authority`
      (`KismetSystemLibrary.K2_SetTimerDelegate` (delegate `ShowVotting`) 1.0))
    (:`Remote`
      _))
  (if (`self.WhiteWin?`)
    ;[1 1 1] First attack
    (`|PlayMontage` (`self.SkeletalMeshWhite`) (`.AttackFigureMontage_9_2F41C3D048E7A7ECB4001CA7344BD301` (break `/Game/Data/Animations/F_FigureAnimations` (`self.WhiteFigureAnimations`)))
      (:`then`
        (`|PlayMontage` (`self.SkeletalMeshBlack`) (`.GetHitMontage_7_C8A06A6549C40A01366E9FAB85831BD4` (break `/Game/Data/Animations/F_FigureAnimations` (`self.BlackFigureAnimations`)))
          (:`OnCompleted`
            (`KismetSystemLibrary.Delay` 1.0)
            ;[1 1 1] Second attack
            (`|PlayMontage` (`self.SkeletalMeshBlack`) (`.AttackFigureMontage_9_2F41C3D048E7A7ECB4001CA7344BD301` (break `/Game/Data/Animations/F_FigureAnimations` (`self.BlackFigureAnimations`)))
              (:`then`
                (`|PlayMontage` (`self.SkeletalMeshWhite`) (`.GetHitMontage_7_C8A06A6549C40A01366E9FAB85831BD4` (break `/Game/Data/Animations/F_FigureAnimations` (`self.WhiteFigureAnimations`)))
                  (:`OnCompleted`
                    (`KismetSystemLibrary.Delay` 1.0)
                    ;[1 1 1] Thirty attack
                    (`|PlayMontage` (`self.SkeletalMeshWhite`) (`.AttackFigureMontage_9_2F41C3D048E7A7ECB4001CA7344BD301` (break `/Game/Data/Animations/F_FigureAnimations` (`self.WhiteFigureAnimations`)))
                      (:`then`
                        (`|PlayMontage` (`self.SkeletalMeshBlack`) (`.GetHitMontage_7_C8A06A6549C40A01366E9FAB85831BD4` (break `/Game/Data/Animations/F_FigureAnimations` (`self.BlackFigureAnimations`)))
                          (:`OnCompleted`
                            (`KismetSystemLibrary.Delay` 1.0)
                            ;[1 1 1] Death and return on battleField
                            (bind _notifyname (`|PlayMontage` (`self.SkeletalMeshBlack`) (`.DeathMontage_11_EBEE7DAD4E65518FCB34098CC58B29E7` (break `/Game/Data/Animations/F_FigureAnimations` (`self.BlackFigureAnimations`))))
                              (:`OnNotifyBegin`
                                (if (== _notifyname "EndMontage")
                                  (`/Engine/EditorBlueprintResources/ActorMacros.Switch Has Authority` :!label _label
                                    (:`Authority`
                                      (if (`|EnumEquality` (`Widget.GetVisibility` (`/Game/Widgets/BattleField/WBP_BattlefieldHUD.WBP_SolutionContinueFight` (`/Game/Blueprints/BattleField/BP_BattleHUD.BattleFieldHUDWidget` (cast `/Game/Blueprints/BattleField/BP_BattleHUD` (`PlayerController.GetHUD` (`self.PlayerController`)) :!pure true)))) "Visible")
                                        (`/Game/Blueprints/BattleField/BP_PCBattle.AllShow/HideWidgetSolutionContinueFight` (`self.PlayerController`) false false "" true))
                                      (cast `/Game/Blueprints/BattleField/PlayerPawn/BP_PlayerArena` (`Controller.K2_GetPawn` (`self.PlayerController`)))
                                      (`/Game/Blueprints/BattleField/BP_PCBattle.RequestOnServerForReturnInBattleField` (`self.PlayerController`)))))))))))))))))))
    (else
      ;[1 1 1] First attack
      (`|PlayMontage` (`self.SkeletalMeshBlack`) (`.AttackFigureMontage_9_2F41C3D048E7A7ECB4001CA7344BD301` (break `/Game/Data/Animations/F_FigureAnimations` (`self.BlackFigureAnimations`)))
        (:`then`
          (`|PlayMontage` (`self.SkeletalMeshWhite`) (`.GetHitMontage_7_C8A06A6549C40A01366E9FAB85831BD4` (break `/Game/Data/Animations/F_FigureAnimations` (`self.WhiteFigureAnimations`)))
            (:`OnCompleted`
              (`KismetSystemLibrary.Delay` 1.0)
              ;[1 1 1] Second attack
              (`|PlayMontage` (`self.SkeletalMeshWhite`) (`.AttackFigureMontage_9_2F41C3D048E7A7ECB4001CA7344BD301` (break `/Game/Data/Animations/F_FigureAnimations` (`self.WhiteFigureAnimations`)))
                (:`then`
                  (`|PlayMontage` (`self.SkeletalMeshBlack`) (`.GetHitMontage_7_C8A06A6549C40A01366E9FAB85831BD4` (break `/Game/Data/Animations/F_FigureAnimations` (`self.BlackFigureAnimations`)))
                    (:`OnCompleted`
                      (`KismetSystemLibrary.Delay` 1.0)
                      ;[1 1 1] Thirty attack
                      (`|PlayMontage` (`self.SkeletalMeshBlack`) (`.AttackFigureMontage_9_2F41C3D048E7A7ECB4001CA7344BD301` (break `/Game/Data/Animations/F_FigureAnimations` (`self.BlackFigureAnimations`)))
                        (:`then`
                          (`|PlayMontage` (`self.SkeletalMeshWhite`) (`.GetHitMontage_7_C8A06A6549C40A01366E9FAB85831BD4` (break `/Game/Data/Animations/F_FigureAnimations` (`self.WhiteFigureAnimations`)))
                            (:`OnCompleted`
                              (`KismetSystemLibrary.Delay` 1.0)
                              ;[1 1 1] Death and return on battleField
                              (bind _notifyname_2 (`|PlayMontage` (`self.SkeletalMeshWhite`) (`.DeathMontage_11_EBEE7DAD4E65518FCB34098CC58B29E7` (break `/Game/Data/Animations/F_FigureAnimations` (`self.WhiteFigureAnimations`))))
                                (:`OnNotifyBegin`
                                  (if (== _notifyname_2 "EndMontage")
                                    (goto _label)))))))))))))))))))

(event `ShowVotting`
  (`/Game/Blueprints/BattleField/BP_PCBattle.AllShow/HideWidgetSolutionContinueFight` (`self.PlayerController`) true false "Skip Fight?" false))

(fn `UserConstructionScript`)