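; Game mode for a chess battle that registers joining players, assigns their colour and removes figures on the server.
; On login it stores the controller, fills the arena fight's controller if unset, then possesses White or Black.
; Colour comes from the saved White player's Steam ID, or the controller's remote role without Steam.
; DestroyFigure acts only on every second call, destroying the figure overlapping the tagged cell after a short delay.
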(event `self.K2_PostLogin`
  (params (NewPlayer :type "PlayerController Object Reference"))
  (bind _asbp_pcbattle (cast `/Game/Blueprints/BattleField/BP_PCBattle` NewPlayer :!pure true))
  (`KismetArrayLibrary.Array_AddUnique` (`self.PlayerControllers`) _asbp_pcbattle)
  (bind _returnvalue (`GameplayStatics.GetActorOfClass` "/Game/Blueprints/BattleField/BP_ArenaFight.BP_ArenaFight_C"))
  (`/Engine/EditorBlueprintResources/StandardMacros.IsValid` (`/Game/Blueprints/BattleField/BP_ArenaFight.PlayerController` _returnvalue)
    (:`Is Valid`
      _)
    (:`Is Not Valid`
      (set `/Game/Blueprints/BattleField/BP_ArenaFight.PlayerController` _asbp_pcbattle _returnvalue)))
  (if (`AdvancedSessionsLibrary.HasOnlineSubsystem` "steam")
    (if (`KismetStringLibrary.EqualEqual_StrStr` (`AdvancedSessionsLibrary.UniqueNetIdToString` (`AdvancedSessionsLibrary.GetUniqueNetIDFromPlayerState` (`Controller.PlayerState` _asbp_pcbattle))) (`.IdPlayerWhiteColorFigures_11_737E70DD4A27F35F14A8D8A6AC69E951` (break `/Game/Data/UI/Structures/F_ColorFiguresPlayersAndId` (`.ColorFigures_7_45CA903548138829D7408A94C10861B6` (break `/Game/Data/UI/Structures/F_GameInformation` (`/Game/Blueprints/BP_GameInstance.GameInformation` (`/Game/Blueprints/Library/BP_FunctionLibrary.GetMyGameInstance`)))))))
      (`/Game/Blueprints/BattleField/BP_PCBattle.StartPossessPlayers` _asbp_pcbattle "White")
      (else
        (`/Game/Blueprints/BattleField/BP_PCBattle.StartPossessPlayers` _asbp_pcbattle "Black")))
    (elif (`|EnumEquality` (`self.GetRemoteRole` _asbp_pcbattle) "ROLE_SimulatedProxy")
      (`/Game/Blueprints/BattleField/BP_PCBattle.StartPossessPlayers` _asbp_pcbattle "White")
      (else
        (`/Game/Blueprints/BattleField/BP_PCBattle.StartPossessPlayers` _asbp_pcbattle "Black")))))

(event `DestroyFigure`
  (params (CellTag :type Name))
  ;[1 1 1] Destroy figure on server
  (`/Engine/EditorBlueprintResources/StandardMacros.FlipFlop`
    (:`B`
      (`KismetSystemLibrary.Delay` 0.2)
      (bind _outactors (`GameplayStatics.GetAllActorsOfClassWithTag` "/Game/Blueprints/BattleField/BP_Cell.BP_Cell_C" CellTag))
      (`self.K2_DestroyActor` (`|GetArrayItem` (`self.GetOverlappingActors` (`|GetArrayItem` _outactors) "/Game/Blueprints/AI/ChessFigure/BP_AIChessFigureBase.BP_AIChessFigureBase_C"))))))

(fn `UserConstructionScript`)