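; BP_Board is the battlefield board, which builds and clears a chess-style 8x8 grid of BP_Cell actors.
; CreateCells, skipped if any cell already exists, spawns 64 attached cells at fixed spacing, each tagged with its square name (a1–h8).
; A FlipFlop alternates two cell materials, which swap at each new row to form the checker pattern.
; DeleteAllCells destroys every BP_Cell in the level, while the construction script does no effective work.
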(fn `CreateCells`
  (locals (LCell :type "/Game/Blueprints/BattleField/BP_Cell Object Reference") (LIndex :type Integer) (LM1 :type "MaterialInterface Object Reference" :default "Material'/Game/Assets/Cells/Materials/M_Cell1.M_Cell1'") (LM2 :type "MaterialInterface Object Reference" :default "Material'/Game/Assets/Cells/Materials/M_Cell2.M_Cell2'") (LCashM :type "MaterialInterface Object Reference"))
  (bind (_returnvalue_x _returnvalue_y _returnvalue_z) (`KismetMathLibrary.BreakVector` (`self.K2_GetActorLocation` self)))
  (bind (_returnvalue_x_2 _returnvalue_y_2 _returnvalue_z_2) (`KismetMathLibrary.BreakVector` (`self.K2_GetActorLocation` self)))
  (bind _cube (`/Game/Blueprints/BattleField/BP_Cell.Cube` (`local.LCell`)))
  (bind _returnvalue (`GameplayStatics.GetActorOfClass` "/Game/Blueprints/BattleField/BP_Cell.BP_Cell_C"))
  (`/Engine/EditorBlueprintResources/StandardMacros.IsValid` _returnvalue
    (:`Is Valid`
      (`KismetSystemLibrary.PrintString` "Ячейка уже есть"))
    (:`Is Not Valid`
      (for _index (range 64)
        (set `local.LIndex` _index)
        (bind _returnvalue_2 (`|SpawnActorFromClass` "/Game/Blueprints/BattleField/BP_Cell.BP_Cell_C" (`KismetMathLibrary.MakeTransform` (0.0 0.0 0.0)) "AlwaysSpawn" "OverrideRootScale" null null))
        (set `local.LCell` _returnvalue_2)
        (`self.K2_AttachToActor` (`local.LCell`) self "None" "SnapToTarget" "SnapToTarget" "SnapToTarget" true)
        (`KismetArrayLibrary.Array_Add` (`Actor.Tags` (`local.LCell`)) (`KismetStringLibrary.Conv_StringToName` (`KismetStringLibrary.Concat_StrStr` (`KismetStringLibrary.Conv_NameToString` (`|GetArrayItem` (`|MakeArray` "a" "b" "c" "d" "e" "f" "g" "h" :!type "Name") (/ (`local.LIndex`) 8))) (`KismetStringLibrary.Conv_IntToString` (+ (mod (`local.LIndex`) 8) 1)))))
        (if (== (mod (`local.LIndex`) 8) 0)
          (`self.K2_SetActorRelativeLocation` (`local.LCell`) (`KismetMathLibrary.MakeVector` 0.0 (`KismetMathLibrary.Conv_IntToDouble` (* (/ (`local.LIndex`) 8) -200)) (+ _returnvalue_z_2 10.0)) false false)
          (set `local.LCashM` (`local.LM1`))
          (set `local.LM1` (`local.LM2`))
          (set `local.LM2` (`local.LCashM`))
          (else
            (`self.K2_SetActorRelativeLocation` (`local.LCell`) (`KismetMathLibrary.MakeVector` (`KismetMathLibrary.Conv_IntToDouble` (* (- (`local.LIndex`) (* (/ (`local.LIndex`) 8) 8)) -200)) (`KismetMathLibrary.Conv_IntToDouble` (* (/ (`local.LIndex`) 8) -200)) (+ _returnvalue_z 10.0)) false false)))
        (`/Engine/EditorBlueprintResources/StandardMacros.FlipFlop`
          (:`A`
            (`PrimitiveComponent.SetMaterial` _cube 0 (`local.LM1`)))
          (:`B`
            (`PrimitiveComponent.SetMaterial` _cube 0 (`local.LM2`))))))))

(fn `DeleteAllCells`
  (bind _outactors (`GameplayStatics.GetAllActorsOfClass` "/Game/Blueprints/BattleField/BP_Cell.BP_Cell_C"))
  (for _array_element _outactors
    (`self.K2_DestroyActor` _array_element)))

(fn `UserConstructionScript`
  (for _ (`self.K2_GetComponentsByClass` "/Script/Engine.ChildActorComponent")
    _))