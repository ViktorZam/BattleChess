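; AI chess bishop that computes its diagonal moves and plays its capture of an enemy piece.
; AttackFigureMulticast sets up both arena fighters, plays the attack montage with notify-driven hit and explosion, then requests the fight view on authority.
; CalculateStepsBishop walks four diagonals using the overlapped cell's algebraic tag, filling AvailableMoves.
; Along each diagonal it also runs check detection, figure disabling and threat-removal cell checks.
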(event `AttackFigureMulticast`
  (params (Target :type "Actor Object Reference"))
  (bind _figureanimations (`self.FigureAnimations`))
  (bind _mesh (`self.Mesh`))
  (bind _asbp_aichess_figure_base (cast `/Game/Blueprints/AI/ChessFigure/BP_AIChessFigureBase` (`|GetArrayItem` (`self.GetOverlappingActors` (cast `/Game/Blueprints/BattleField/BP_Cell` Target :!pure true) "/Game/Blueprints/AI/ChessFigure/BP_AIChessFigureBase.BP_AIChessFigureBase_C")) :!pure true))
  (bind _figureanimations_2 (`/Game/Blueprints/AI/ChessFigure/BP_AIChessFigureBase.FigureAnimations` _asbp_aichess_figure_base))
  (bind _mesh_2 (`Character.Mesh` _asbp_aichess_figure_base))
  ;[1 1 1] Set arena fight And Attack enemy figure on battlefield
  (if (== (`|GetArrayItem` (`self.Tags`)) "White")
    (`self.Set Arena Figures` _figureanimations _figureanimations_2 true _mesh _mesh_2)
    (else
      (`self.Set Arena Figures` _figureanimations_2 _figureanimations false _mesh_2 _mesh)))
  (bind _notifyname (`|PlayMontage` (`self.Mesh`) (`.AttackFigureMontage_9_2F41C3D048E7A7ECB4001CA7344BD301` (break `/Game/Data/Animations/F_FigureAnimations` (`self.FigureAnimations`))))
    (:`OnCompleted`
      (`/Engine/EditorBlueprintResources/StandardMacros.IsValid` (`self.PlayerController`)
        (:`Is Valid`
          (`/Engine/EditorBlueprintResources/ActorMacros.Switch Has Authority`
            (:`Authority`
              (`self.RequestShowFight`))))))
    (:`OnNotifyBegin`
      (if (== _notifyname "EnemyGetHit")
        (`self.GetHit` _asbp_aichess_figure_base)
        (`GameplayStatics.SpawnEmitterAtLocation` "/Game/Assets/VFX/P_ky_explosion.P_ky_explosion" (+ (* (`self.GetActorForwardVector` self) 200.0) (`self.K2_GetActorLocation` self)) (struct) (2.0 2.0 2.0))))))

(event `/Game/Blueprints/Interfaces/BPI_Figures.AttackFigure`
  (params (TargetForAttack :type "Actor Object Reference"))
  ;[1 1 1] Set arena fight And Attack enemy figure on battlefield
  (`self.AttackFigureMulticast` TargetForAttack))

(event `/Game/Blueprints/Interfaces/BPI_Figures.CalculateCheck/DisableFigures`
  (params (Attacker :type "/Game/Blueprints/AI/ChessFigure/BP_AIChessFigureBase Object Reference") (CellsOfAttacker :type "Array of Name (by ref)") (CellsRemoveThreat :type "Array of String (by ref)"))
  (`self.CalculateStepsBishop` Attacker CellsOfAttacker CellsRemoveThreat))

(fn `CalculateStepsBishop`
  (params (Attacker :type "/Game/Blueprints/AI/ChessFigure/BP_AIChessFigureBase Object Reference") (CellsOfAttacker :type "Array of Name (by ref)") (CellsRemoveThreat :type "Array of String (by ref)"))
  (locals (LPositionCell :type Name) (LDisableFigure :type "Array of /Game/Blueprints/AI/ChessFigure/BP_AIChessFigureBase Object Reference") (LDifferenceSignAndNumberInPosition :type Integer))
  (bind _array (`|MakeArray` "a" "b" "c" "d" "e" "f" "g" "h"))
  (bind _array_2 (`|MakeArray` "a" "b" "c" "d" "e" "f" "g" "h"))
  (bind _returnvalue (`KismetStringLibrary.Conv_StringToInt` (`KismetStringLibrary.GetSubstring` (`KismetStringLibrary.Conv_NameToString` (`local.LPositionCell`)) 1)))
  (bind _returnvalue_2 (`KismetStringLibrary.Conv_StringToInt` (`KismetStringLibrary.GetSubstring` (`KismetStringLibrary.Conv_NameToString` (`local.LPositionCell`)) 1)))
  (bind _returnvalue_3 (- 8 (`KismetStringLibrary.Conv_StringToInt` (`KismetStringLibrary.GetSubstring` (`KismetStringLibrary.Conv_NameToString` (`local.LPositionCell`)) 1))))
  (bind _returnvalue_4 (- 8 (`KismetStringLibrary.Conv_StringToInt` (`KismetStringLibrary.GetSubstring` (`KismetStringLibrary.Conv_NameToString` (`local.LPositionCell`)) 1))))
  (bind _returnvalue_5 (+ (`KismetArrayLibrary.Array_Find` (`|MakeArray` "h" "g" "f" "e" "d" "c" "b" "a") (`KismetStringLibrary.GetSubstring` (`KismetStringLibrary.Conv_NameToString` (`local.LPositionCell`)))) 1))
  (bind _returnvalue_6 (+ (`KismetArrayLibrary.Array_Find` (`|MakeArray` "a" "b" "c" "d" "e" "f" "g" "h") (`KismetStringLibrary.GetSubstring` (`KismetStringLibrary.Conv_NameToString` (`local.LPositionCell`)))) 1))
  (bind _returnvalue_7 (+ (`KismetArrayLibrary.Array_Find` (`|MakeArray` "a" "b" "c" "d" "e" "f" "g" "h") (`KismetStringLibrary.GetSubstring` (`KismetStringLibrary.Conv_NameToString` (`local.LPositionCell`)))) 1))
  (bind _returnvalue_8 (- 8 _returnvalue_5))
  (bind _returnvalue_9 (- 8 _returnvalue_7))
  (bind _returnvalue_10 (- 9 (+ (`KismetArrayLibrary.Array_Find` (`|MakeArray` "a" "b" "c" "d" "e" "f" "g" "h") (`KismetStringLibrary.GetSubstring` (`KismetStringLibrary.Conv_NameToString` (`local.LPositionCell`)))) 1)))
  (set `local.LPositionCell` (`|GetArrayItem` (`Actor.Tags` (`|GetArrayItem` (`self.GetOverlappingActors` "/Game/Blueprints/BattleField/BP_Cell.BP_Cell_C")))))
  (for _index (range 4)
    (switch `int` _index
      (:`0`
        ;[1 1 1] Up-Right
        (`/Engine/EditorBlueprintResources/StandardMacros.CompareInt` _returnvalue_3 _returnvalue_9
          (:`>`
            (set `local.LDifferenceSignAndNumberInPosition` (- _returnvalue_3 _returnvalue_9))
            (for _index_2 (range _returnvalue_7 9)
              (bind _returnvalue_11 (`KismetStringLibrary.Conv_StringToName` (`KismetStringLibrary.Concat_StrStr` (`KismetStringLibrary.GetSubstring` (`|GetArrayItem` (`|MakeArray` "a" "b" "c" "d" "e" "f" "g" "h") (- _index_2 1))) (`KismetStringLibrary.Conv_IntToString` (- _index_2 (`local.LDifferenceSignAndNumberInPosition`))))))
              (`KismetArrayLibrary.Array_AddUnique` (`self.AvailableMoves`) _returnvalue_11)
              (`self.CalculateCheck/FindFigureForDisable` _returnvalue_11 (`local.LPositionCell`) (`local.LDisableFigure`) true (`local.Attacker`) (`local.CellsOfAttacker`) (`local.CellsRemoveThreat`)))
            (`self.DisableFigure` (`local.LDisableFigure`))
            (`self.Check Cells Remove Threat` (`local.Attacker`) (`local.CellsRemoveThreat`)))
          (:`==`
            (set `local.LDifferenceSignAndNumberInPosition` (- _returnvalue_9 _returnvalue_3) :!label _label)
            (for _index_3 (range (`KismetStringLibrary.Conv_StringToInt` (`KismetStringLibrary.GetSubstring` (`KismetStringLibrary.Conv_NameToString` (`local.LPositionCell`)) 1)) 9)
              (bind _returnvalue_12 (`KismetStringLibrary.Conv_StringToName` (`KismetStringLibrary.Concat_StrStr` (`KismetStringLibrary.GetSubstring` (`|GetArrayItem` (`|MakeArray` "a" "b" "c" "d" "e" "f" "g" "h") (- (- _index_3 (`local.LDifferenceSignAndNumberInPosition`)) 1))) (`KismetStringLibrary.Conv_IntToString` _index_3))))
              (`KismetArrayLibrary.Array_AddUnique` (`self.AvailableMoves`) _returnvalue_12)
              (`self.CalculateCheck/FindFigureForDisable` _returnvalue_12 (`local.LPositionCell`) (`local.LDisableFigure`) true (`local.Attacker`) (`local.CellsOfAttacker`) (`local.CellsRemoveThreat`)))
            (`self.DisableFigure` (`local.LDisableFigure`))
            (`self.Check Cells Remove Threat` (`local.Attacker`) (`local.CellsRemoveThreat`)))
          (:`<`
            (goto _label))))
      (:`1`
        ;[1 1 1] Right-Down
        (`/Engine/EditorBlueprintResources/StandardMacros.CompareInt` _returnvalue_2 _returnvalue_10
          (:`>`
            (set `local.LDifferenceSignAndNumberInPosition` (- _returnvalue_2 _returnvalue_10))
            (for _index_4 (range (* _returnvalue_10 -1) 0)
              (bind _returnvalue_13 (* _index_4 -1))
              (bind _returnvalue_14 (`KismetStringLibrary.Conv_StringToName` (`KismetStringLibrary.Concat_StrStr` (`KismetStringLibrary.GetSubstring` (`|GetArrayItem` _array (- (+ (`KismetArrayLibrary.Array_LastIndex` _array) 1) _returnvalue_13))) (`KismetStringLibrary.Conv_IntToString` (+ _returnvalue_13 (`local.LDifferenceSignAndNumberInPosition`))))))
              (`KismetArrayLibrary.Array_AddUnique` (`self.AvailableMoves`) _returnvalue_14)
              (`self.CalculateCheck/FindFigureForDisable` _returnvalue_14 (`local.LPositionCell`) (`local.LDisableFigure`) true (`local.Attacker`) (`local.CellsOfAttacker`) (`local.CellsRemoveThreat`)))
            (`self.DisableFigure` (`local.LDisableFigure`))
            (`self.Check Cells Remove Threat` (`local.Attacker`) (`local.CellsRemoveThreat`)))
          (:`==`
            (set `local.LDifferenceSignAndNumberInPosition` (- _returnvalue_10 _returnvalue_2) :!label _label_2)
            (for _index_5 (range (* (`KismetStringLibrary.Conv_StringToInt` (`KismetStringLibrary.GetSubstring` (`KismetStringLibrary.Conv_NameToString` (`local.LPositionCell`)) 1)) -1) 0)
              (bind _returnvalue_15 (* _index_5 -1))
              (bind _returnvalue_16 (`KismetStringLibrary.Conv_StringToName` (`KismetStringLibrary.Concat_StrStr` (`KismetStringLibrary.GetSubstring` (`|GetArrayItem` _array_2 (- (+ (`KismetArrayLibrary.Array_LastIndex` _array_2) 1) (+ _returnvalue_15 (`local.LDifferenceSignAndNumberInPosition`))))) (`KismetStringLibrary.Conv_IntToString` _returnvalue_15))))
              (`KismetArrayLibrary.Array_AddUnique` (`self.AvailableMoves`) _returnvalue_16)
              (`self.CalculateCheck/FindFigureForDisable` _returnvalue_16 (`local.LPositionCell`) (`local.LDisableFigure`) true (`local.Attacker`) (`local.CellsOfAttacker`) (`local.CellsRemoveThreat`)))
            (`self.DisableFigure` (`local.LDisableFigure`))
            (`self.Check Cells Remove Threat` (`local.Attacker`) (`local.CellsRemoveThreat`)))
          (:`<`
            (goto _label_2))))
      (:`2`
        ;[1 1 1] Left-Down
        (`/Engine/EditorBlueprintResources/StandardMacros.CompareInt` _returnvalue _returnvalue_6
          (:`>`
            (set `local.LDifferenceSignAndNumberInPosition` (- _returnvalue _returnvalue_6))
            (for _index_6 (range (* _returnvalue_6 -1) 0)
              (bind _returnvalue_17 (* _index_6 -1))
              (bind _returnvalue_18 (`KismetStringLibrary.Conv_StringToName` (`KismetStringLibrary.Concat_StrStr` (`KismetStringLibrary.GetSubstring` (`|GetArrayItem` (`|MakeArray` "a" "b" "c" "d" "e" "f" "g" "h") (- _returnvalue_17 1))) (`KismetStringLibrary.Conv_IntToString` (+ _returnvalue_17 (`local.LDifferenceSignAndNumberInPosition`))))))
              (`KismetArrayLibrary.Array_AddUnique` (`self.AvailableMoves`) _returnvalue_18)
              (`self.CalculateCheck/FindFigureForDisable` _returnvalue_18 (`local.LPositionCell`) (`local.LDisableFigure`) true (`local.Attacker`) (`local.CellsOfAttacker`) (`local.CellsRemoveThreat`)))
            (`self.DisableFigure` (`local.LDisableFigure`))
            (`self.Check Cells Remove Threat` (`local.Attacker`) (`local.CellsRemoveThreat`)))
          (:`==`
            (set `local.LDifferenceSignAndNumberInPosition` (- _returnvalue_6 _returnvalue) :!label _label_3)
            (for _index_7 (range (* (`KismetStringLibrary.Conv_StringToInt` (`KismetStringLibrary.GetSubstring` (`KismetStringLibrary.Conv_NameToString` (`local.LPositionCell`)) 1)) -1) 0)
              (bind _returnvalue_19 (* _index_7 -1))
              (bind _returnvalue_20 (`KismetStringLibrary.Conv_StringToName` (`KismetStringLibrary.Concat_StrStr` (`KismetStringLibrary.GetSubstring` (`|GetArrayItem` (`|MakeArray` "a" "b" "c" "d" "e" "f" "g" "h") (- (+ _returnvalue_19 (`local.LDifferenceSignAndNumberInPosition`)) 1))) (`KismetStringLibrary.Conv_IntToString` _returnvalue_19))))
              (`KismetArrayLibrary.Array_AddUnique` (`self.AvailableMoves`) _returnvalue_20)
              (`self.CalculateCheck/FindFigureForDisable` _returnvalue_20 (`local.LPositionCell`) (`local.LDisableFigure`) true (`local.Attacker`) (`local.CellsOfAttacker`) (`local.CellsRemoveThreat`)))
            (`self.DisableFigure` (`local.LDisableFigure`))
            (`self.Check Cells Remove Threat` (`local.Attacker`) (`local.CellsRemoveThreat`)))
          (:`<`
            (goto _label_3))))
      (:`3`
        ;[1 1 1] Up-Left
        (`/Engine/EditorBlueprintResources/StandardMacros.CompareInt` _returnvalue_4 _returnvalue_8
          (:`>`
            (set `local.LDifferenceSignAndNumberInPosition` (- _returnvalue_4 _returnvalue_8))
            (for _index_8 (range _returnvalue_5 9)
              (bind _returnvalue_21 (`KismetStringLibrary.Conv_StringToName` (`KismetStringLibrary.Concat_StrStr` (`KismetStringLibrary.GetSubstring` (`|GetArrayItem` (`|MakeArray` "h" "g" "f" "e" "d" "c" "b" "a") (- _index_8 1))) (`KismetStringLibrary.Conv_IntToString` (- _index_8 (`local.LDifferenceSignAndNumberInPosition`))))))
              (`KismetArrayLibrary.Array_AddUnique` (`self.AvailableMoves`) _returnvalue_21)
              (`self.CalculateCheck/FindFigureForDisable` _returnvalue_21 (`local.LPositionCell`) (`local.LDisableFigure`) true (`local.Attacker`) (`local.CellsOfAttacker`) (`local.CellsRemoveThreat`)))
            (`self.DisableFigure` (`local.LDisableFigure`))
            (`self.Check Cells Remove Threat` (`local.Attacker`) (`local.CellsRemoveThreat`)))
          (:`==`
            (set `local.LDifferenceSignAndNumberInPosition` (- _returnvalue_8 _returnvalue_4) :!label _label_4)
            (for _index_9 (range (`KismetStringLibrary.Conv_StringToInt` (`KismetStringLibrary.GetSubstring` (`KismetStringLibrary.Conv_NameToString` (`local.LPositionCell`)) 1)) 9)
              (bind _returnvalue_22 (`KismetStringLibrary.Conv_StringToName` (`KismetStringLibrary.Concat_StrStr` (`KismetStringLibrary.GetSubstring` (`|GetArrayItem` (`|MakeArray` "h" "g" "f" "e" "d" "c" "b" "a") (- (- _index_9 (`local.LDifferenceSignAndNumberInPosition`)) 1))) (`KismetStringLibrary.Conv_IntToString` _index_9))))
              (`KismetArrayLibrary.Array_AddUnique` (`self.AvailableMoves`) _returnvalue_22)
              (`self.CalculateCheck/FindFigureForDisable` _returnvalue_22 (`local.LPositionCell`) (`local.LDisableFigure`) true (`local.Attacker`) (`local.CellsOfAttacker`) (`local.CellsRemoveThreat`)))
            (`self.DisableFigure` (`local.LDisableFigure`))
            (`self.Check Cells Remove Threat` (`local.Attacker`) (`local.CellsRemoveThreat`)))
          (:`<`
            (goto _label_4)))))))

(fn `UserConstructionScript`
  (`parent.UserConstructionScript`))