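; AI chess knight figure that computes its L-shaped moves when the CalculateCheck/DisableFigures event fires.
; It reads its square from the tag of the overlapping BP_Cell and tests the eight jumps against board bounds using file-letter and rank math.
; Each valid square joins AvailableMoves and feeds CalculateCheckFindFigureForDisable, DisableFigure and CheckCellsRemoveThreat, which receive the attacker and threat-removal data as applicable.
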(event `/Game/Blueprints/Interfaces/BPI_Figures.CalculateCheck/DisableFigures`
  (params (Attacker :type "/Game/Blueprints/AI/ChessFigure/BP_AIChessFigureBase Object Reference") (CellsOfAttacker :type "Array of Name (by ref)") (CellsRemoveThreat :type "Array of String (by ref)"))
  (`self.CalculateStepsKnight` Attacker CellsOfAttacker CellsRemoveThreat))

(fn `CalculateStepsKnight`
  (params (Attacker :type "/Game/Blueprints/AI/ChessFigure/BP_AIChessFigureBase Object Reference") (CellsOfAttacker :type "Array of Name (by ref)") (CellsRemoveThreat :type "Array of String (by ref)"))
  (locals (LPositionCell :type Name) (LDisableFigure :type "Array of /Game/Blueprints/AI/ChessFigure/BP_AIChessFigureBase Object Reference") (LDifferenceSignAndNumberInPosition :type Integer))
  (bind _returnvalue (`KismetStringLibrary.Conv_StringToName` (`KismetStringLibrary.Concat_StrStr` (`|GetArrayItem` (`|MakeArray` "a" "b" "c" "d" "e" "f" "g" "h") (+ (`KismetArrayLibrary.Array_Find` (`|MakeArray` "a" "b" "c" "d" "e" "f" "g" "h") (`KismetStringLibrary.GetSubstring` (`KismetStringLibrary.Conv_NameToString` (`local.LPositionCell`)))) 1)) (`KismetStringLibrary.Conv_IntToString` (- (`KismetStringLibrary.Conv_StringToInt` (`KismetStringLibrary.GetSubstring` (`KismetStringLibrary.Conv_NameToString` (`local.LPositionCell`)) 1)) 1)))))
  (bind _returnvalue_2 (`KismetStringLibrary.Conv_StringToName` (`KismetStringLibrary.Concat_StrStr` (`|GetArrayItem` (`|MakeArray` "a" "b" "c" "d" "e" "f" "g" "h") (+ (`KismetArrayLibrary.Array_Find` (`|MakeArray` "a" "b" "c" "d" "e" "f" "g" "h") (`KismetStringLibrary.GetSubstring` (`KismetStringLibrary.Conv_NameToString` (`local.LPositionCell`)))) 1)) (`KismetStringLibrary.Conv_IntToString` (- (`KismetStringLibrary.Conv_StringToInt` (`KismetStringLibrary.GetSubstring` (`KismetStringLibrary.Conv_NameToString` (`local.LPositionCell`)) 1)) 2)))))
  (bind _returnvalue_3 (`KismetStringLibrary.Conv_StringToName` (`KismetStringLibrary.Concat_StrStr` (`|GetArrayItem` (`|MakeArray` "a" "b" "c" "d" "e" "f" "g" "h") (- (`KismetArrayLibrary.Array_Find` (`|MakeArray` "a" "b" "c" "d" "e" "f" "g" "h") (`KismetStringLibrary.GetSubstring` (`KismetStringLibrary.Conv_NameToString` (`local.LPositionCell`)))) 1)) (`KismetStringLibrary.Conv_IntToString` (- (`KismetStringLibrary.Conv_StringToInt` (`KismetStringLibrary.GetSubstring` (`KismetStringLibrary.Conv_NameToString` (`local.LPositionCell`)) 1)) 2)))))
  (bind _returnvalue_4 (`KismetStringLibrary.Conv_StringToName` (`KismetStringLibrary.Concat_StrStr` (`|GetArrayItem` (`|MakeArray` "a" "b" "c" "d" "e" "f" "g" "h") (- (`KismetArrayLibrary.Array_Find` (`|MakeArray` "a" "b" "c" "d" "e" "f" "g" "h") (`KismetStringLibrary.GetSubstring` (`KismetStringLibrary.Conv_NameToString` (`local.LPositionCell`)))) 2)) (`KismetStringLibrary.Conv_IntToString` (- (`KismetStringLibrary.Conv_StringToInt` (`KismetStringLibrary.GetSubstring` (`KismetStringLibrary.Conv_NameToString` (`local.LPositionCell`)) 1)) 1)))))
  (bind _returnvalue_5 (`KismetStringLibrary.Conv_StringToName` (`KismetStringLibrary.Concat_StrStr` (`|GetArrayItem` (`|MakeArray` "a" "b" "c" "d" "e" "f" "g" "h") (- (`KismetArrayLibrary.Array_Find` (`|MakeArray` "a" "b" "c" "d" "e" "f" "g" "h") (`KismetStringLibrary.GetSubstring` (`KismetStringLibrary.Conv_NameToString` (`local.LPositionCell`)))) 2)) (`KismetStringLibrary.Conv_IntToString` (+ (`KismetStringLibrary.Conv_StringToInt` (`KismetStringLibrary.GetSubstring` (`KismetStringLibrary.Conv_NameToString` (`local.LPositionCell`)) 1)) 1)))))
  (bind _returnvalue_6 (`KismetStringLibrary.Conv_StringToName` (`KismetStringLibrary.Concat_StrStr` (`|GetArrayItem` (`|MakeArray` "a" "b" "c" "d" "e" "f" "g" "h") (+ (`KismetArrayLibrary.Array_Find` (`|MakeArray` "a" "b" "c" "d" "e" "f" "g" "h") (`KismetStringLibrary.GetSubstring` (`KismetStringLibrary.Conv_NameToString` (`local.LPositionCell`)))) 1)) (`KismetStringLibrary.Conv_IntToString` (+ (`KismetStringLibrary.Conv_StringToInt` (`KismetStringLibrary.GetSubstring` (`KismetStringLibrary.Conv_NameToString` (`local.LPositionCell`)) 1)) 2)))))
  (bind _returnvalue_7 (`KismetStringLibrary.Conv_StringToName` (`KismetStringLibrary.Concat_StrStr` (`|GetArrayItem` (`|MakeArray` "a" "b" "c" "d" "e" "f" "g" "h") (- (`KismetArrayLibrary.Array_Find` (`|MakeArray` "a" "b" "c" "d" "e" "f" "g" "h") (`KismetStringLibrary.GetSubstring` (`KismetStringLibrary.Conv_NameToString` (`local.LPositionCell`)))) 1)) (`KismetStringLibrary.Conv_IntToString` (+ (`KismetStringLibrary.Conv_StringToInt` (`KismetStringLibrary.GetSubstring` (`KismetStringLibrary.Conv_NameToString` (`local.LPositionCell`)) 1)) 2)))))
  (bind _returnvalue_8 (`KismetStringLibrary.Conv_StringToName` (`KismetStringLibrary.Concat_StrStr` (`|GetArrayItem` (`|MakeArray` "a" "b" "c" "d" "e" "f" "g" "h") (+ (`KismetArrayLibrary.Array_Find` (`|MakeArray` "a" "b" "c" "d" "e" "f" "g" "h") (`KismetStringLibrary.GetSubstring` (`KismetStringLibrary.Conv_NameToString` (`local.LPositionCell`)))) 2)) (`KismetStringLibrary.Conv_IntToString` (+ (`KismetStringLibrary.Conv_StringToInt` (`KismetStringLibrary.GetSubstring` (`KismetStringLibrary.Conv_NameToString` (`local.LPositionCell`)) 1)) 1)))))
  (set `local.LPositionCell` (`|GetArrayItem` (`Actor.Tags` (`|GetArrayItem` (`self.GetOverlappingActors` "/Game/Blueprints/BattleField/BP_Cell.BP_Cell_C")))))
  (for _index (range 8)
    (switch `int` _index
      (:`0`
        ;[1 1 1] Up-Right
        (`/Engine/EditorBlueprintResources/StandardMacros.CompareInt` (+ (`KismetStringLibrary.Conv_StringToInt` (`KismetStringLibrary.GetSubstring` (`KismetStringLibrary.Conv_NameToString` (`local.LPositionCell`)) 1)) 2) 8
          (:`==`
            _)
          (:`<`
            _))
        (`/Engine/EditorBlueprintResources/StandardMacros.CompareInt` (+ (`KismetArrayLibrary.Array_Find` (`|MakeArray` "a" "b" "c" "d" "e" "f" "g" "h") (`KismetStringLibrary.GetSubstring` (`KismetStringLibrary.Conv_NameToString` (`local.LPositionCell`)))) 1) 7
          (:`==`
            _)
          (:`<`
            _))
        (`KismetArrayLibrary.Array_AddUnique` (`self.AvailableMoves`) _returnvalue_6)
        (`self.CalculateCheck/FindFigureForDisable` _returnvalue_6 (`local.LPositionCell`) (`local.LDisableFigure`) true (`local.Attacker`) (`local.CellsOfAttacker`) (`local.CellsRemoveThreat`))
        (`self.DisableFigure` (`local.LDisableFigure`))
        (`self.Check Cells Remove Threat` (`local.Attacker`) (`local.CellsRemoveThreat`)))
      (:`1`
        ;[1 1 1] Right-Up
        (`/Engine/EditorBlueprintResources/StandardMacros.CompareInt` (+ (`KismetStringLibrary.Conv_StringToInt` (`KismetStringLibrary.GetSubstring` (`KismetStringLibrary.Conv_NameToString` (`local.LPositionCell`)) 1)) 1) 8
          (:`==`
            _)
          (:`<`
            _))
        (`/Engine/EditorBlueprintResources/StandardMacros.CompareInt` (+ (`KismetArrayLibrary.Array_Find` (`|MakeArray` "a" "b" "c" "d" "e" "f" "g" "h") (`KismetStringLibrary.GetSubstring` (`KismetStringLibrary.Conv_NameToString` (`local.LPositionCell`)))) 2) 7
          (:`==`
            _)
          (:`<`
            _))
        (`KismetArrayLibrary.Array_AddUnique` (`self.AvailableMoves`) _returnvalue_8)
        (`self.CalculateCheck/FindFigureForDisable` _returnvalue_8 (`local.LPositionCell`) (`local.LDisableFigure`) true (`local.Attacker`) (`local.CellsOfAttacker`) (`local.CellsRemoveThreat`))
        (`self.DisableFigure` (`local.LDisableFigure`))
        (`self.Check Cells Remove Threat` (`local.Attacker`) (`local.CellsRemoveThreat`)))
      (:`2`
        ;[1 1 1] Right-Down
        (`/Engine/EditorBlueprintResources/StandardMacros.CompareInt` (- (`KismetStringLibrary.Conv_StringToInt` (`KismetStringLibrary.GetSubstring` (`KismetStringLibrary.Conv_NameToString` (`local.LPositionCell`)) 1)) 1) 1
          (:`>`
            _)
          (:`==`
            _))
        (`/Engine/EditorBlueprintResources/StandardMacros.CompareInt` (+ (`KismetArrayLibrary.Array_Find` (`|MakeArray` "a" "b" "c" "d" "e" "f" "g" "h") (`KismetStringLibrary.GetSubstring` (`KismetStringLibrary.Conv_NameToString` (`local.LPositionCell`)))) 1) 7
          (:`==`
            _)
          (:`<`
            _))
        (`KismetArrayLibrary.Array_AddUnique` (`self.AvailableMoves`) _returnvalue)
        (`self.CalculateCheck/FindFigureForDisable` _returnvalue (`local.LPositionCell`) (`local.LDisableFigure`) true (`local.Attacker`) (`local.CellsOfAttacker`) (`local.CellsRemoveThreat`))
        (`self.DisableFigure` (`local.LDisableFigure`))
        (`self.Check Cells Remove Threat` (`local.Attacker`) (`local.CellsRemoveThreat`)))
      (:`3`
        ;[1 1 1] Down-Right
        (`/Engine/EditorBlueprintResources/StandardMacros.CompareInt` (- (`KismetStringLibrary.Conv_StringToInt` (`KismetStringLibrary.GetSubstring` (`KismetStringLibrary.Conv_NameToString` (`local.LPositionCell`)) 1)) 2) 1
          (:`>`
            _)
          (:`==`
            _))
        (`/Engine/EditorBlueprintResources/StandardMacros.CompareInt` (+ (`KismetArrayLibrary.Array_Find` (`|MakeArray` "a" "b" "c" "d" "e" "f" "g" "h") (`KismetStringLibrary.GetSubstring` (`KismetStringLibrary.Conv_NameToString` (`local.LPositionCell`)))) 1) 7
          (:`==`
            _)
          (:`<`
            _))
        (`KismetArrayLibrary.Array_AddUnique` (`self.AvailableMoves`) _returnvalue_2)
        (`self.CalculateCheck/FindFigureForDisable` _returnvalue_2 (`local.LPositionCell`) (`local.LDisableFigure`) true (`local.Attacker`) (`local.CellsOfAttacker`) (`local.CellsRemoveThreat`))
        (`self.DisableFigure` (`local.LDisableFigure`))
        (`self.Check Cells Remove Threat` (`local.Attacker`) (`local.CellsRemoveThreat`)))
      (:`4`
        ;[1 1 1] Down-Left
        (`/Engine/EditorBlueprintResources/StandardMacros.CompareInt` (- (`KismetStringLibrary.Conv_StringToInt` (`KismetStringLibrary.GetSubstring` (`KismetStringLibrary.Conv_NameToString` (`local.LPositionCell`)) 1)) 2) 1
          (:`>`
            _)
          (:`==`
            _))
        (`/Engine/EditorBlueprintResources/StandardMacros.CompareInt` (- (`KismetArrayLibrary.Array_Find` (`|MakeArray` "a" "b" "c" "d" "e" "f" "g" "h") (`KismetStringLibrary.GetSubstring` (`KismetStringLibrary.Conv_NameToString` (`local.LPositionCell`)))) 1)
          (:`>`
            _)
          (:`==`
            _))
        (`KismetArrayLibrary.Array_AddUnique` (`self.AvailableMoves`) _returnvalue_3)
        (`self.CalculateCheck/FindFigureForDisable` _returnvalue_3 (`local.LPositionCell`) (`local.LDisableFigure`) true (`local.Attacker`) (`local.CellsOfAttacker`) (`local.CellsRemoveThreat`))
        (`self.DisableFigure` (`local.LDisableFigure`))
        (`self.Check Cells Remove Threat` (`local.Attacker`) (`local.CellsRemoveThreat`)))
      (:`5`
        ;[1 1 1] Left-Down
        (`/Engine/EditorBlueprintResources/StandardMacros.CompareInt` (- (`KismetStringLibrary.Conv_StringToInt` (`KismetStringLibrary.GetSubstring` (`KismetStringLibrary.Conv_NameToString` (`local.LPositionCell`)) 1)) 1) 1
          (:`>`
            _)
          (:`==`
            _))
        (`/Engine/EditorBlueprintResources/StandardMacros.CompareInt` (- (`KismetArrayLibrary.Array_Find` (`|MakeArray` "a" "b" "c" "d" "e" "f" "g" "h") (`KismetStringLibrary.GetSubstring` (`KismetStringLibrary.Conv_NameToString` (`local.LPositionCell`)))) 2)
          (:`>`
            _)
          (:`==`
            _))
        (`KismetArrayLibrary.Array_AddUnique` (`self.AvailableMoves`) _returnvalue_4)
        (`self.CalculateCheck/FindFigureForDisable` _returnvalue_4 (`local.LPositionCell`) (`local.LDisableFigure`) true (`local.Attacker`) (`local.CellsOfAttacker`) (`local.CellsRemoveThreat`))
        (`self.DisableFigure` (`local.LDisableFigure`))
        (`self.Check Cells Remove Threat` (`local.Attacker`) (`local.CellsRemoveThreat`)))
      (:`6`
        ;[1 1 1] Left-Up
        (`/Engine/EditorBlueprintResources/StandardMacros.CompareInt` (+ (`KismetStringLibrary.Conv_StringToInt` (`KismetStringLibrary.GetSubstring` (`KismetStringLibrary.Conv_NameToString` (`local.LPositionCell`)) 1)) 1) 8
          (:`==`
            _)
          (:`<`
            _))
        (`/Engine/EditorBlueprintResources/StandardMacros.CompareInt` (- (`KismetArrayLibrary.Array_Find` (`|MakeArray` "a" "b" "c" "d" "e" "f" "g" "h") (`KismetStringLibrary.GetSubstring` (`KismetStringLibrary.Conv_NameToString` (`local.LPositionCell`)))) 2)
          (:`>`
            _)
          (:`==`
            _))
        (`KismetArrayLibrary.Array_AddUnique` (`self.AvailableMoves`) _returnvalue_5)
        (`self.CalculateCheck/FindFigureForDisable` _returnvalue_5 (`local.LPositionCell`) (`local.LDisableFigure`) true (`local.Attacker`) (`local.CellsOfAttacker`) (`local.CellsRemoveThreat`))
        (`self.DisableFigure` (`local.LDisableFigure`))
        (`self.Check Cells Remove Threat` (`local.Attacker`) (`local.CellsRemoveThreat`)))
      (:`7`
        ;[1 1 1] Up-Left
        (`/Engine/EditorBlueprintResources/StandardMacros.CompareInt` (+ (`KismetStringLibrary.Conv_StringToInt` (`KismetStringLibrary.GetSubstring` (`KismetStringLibrary.Conv_NameToString` (`local.LPositionCell`)) 1)) 2) 8
          (:`==`
            _)
          (:`<`
            _))
        (`/Engine/EditorBlueprintResources/StandardMacros.CompareInt` (- (`KismetArrayLibrary.Array_Find` (`|MakeArray` "a" "b" "c" "d" "e" "f" "g" "h") (`KismetStringLibrary.GetSubstring` (`KismetStringLibrary.Conv_NameToString` (`local.LPositionCell`)))) 1)
          (:`>`
            _)
          (:`==`
            _))
        (`KismetArrayLibrary.Array_AddUnique` (`self.AvailableMoves`) _returnvalue_7)
        (`self.CalculateCheck/FindFigureForDisable` _returnvalue_7 (`local.LPositionCell`) (`local.LDisableFigure`) true (`local.Attacker`) (`local.CellsOfAttacker`) (`local.CellsRemoveThreat`))
        (`self.DisableFigure` (`local.LDisableFigure`))
        (`self.Check Cells Remove Threat` (`local.Attacker`) (`local.CellsRemoveThreat`))))))

(fn `UserConstructionScript`
  (`parent.UserConstructionScript`))