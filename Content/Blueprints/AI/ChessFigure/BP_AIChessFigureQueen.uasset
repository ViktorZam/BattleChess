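; AI queen chess piece that works out its available moves and runs check and figure-disabling calculations.
; On CalculateCheck/DisableFigures, it reads its square from the overlapped BP_Cell's tag and walks eight directions to the board edge, building cell names through file-letter and rank arithmetic.
; Each square joins AvailableMoves and goes to CalculateCheckFindFigureForDisable.
; Each direction ends with DisableFigure and CheckCellsRemoveThreat, except one up-right branch, which omits the latter.
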(event `self.ReceiveBeginPlay`
  (`parent.ReceiveBeginPlay`))

(event `self.ReceiveTick`
  (params (DeltaSeconds :type "Float (single-precision)")))

(event `/Game/Blueprints/Interfaces/BPI_Figures.CalculateCheck/DisableFigures`
  (params (Attacker :type "/Game/Blueprints/AI/ChessFigure/BP_AIChessFigureBase Object Reference") (CellsOfAttacker :type "Array of Name (by ref)") (CellsRemoveThreat :type "Array of String (by ref)"))
  (`self.Calculate Steps Queen` Attacker CellsOfAttacker CellsRemoveThreat))

(fn `Calculate Steps Queen`
  (params (Attacker :type "/Game/Blueprints/AI/ChessFigure/BP_AIChessFigureBase Object Reference") (CellsOfAttacker :type "Array of Name (by ref)") (CellsRemoveThreat :type "Array of String (by ref)"))
  (locals (LPositionCell :type Name) (LDisableFigure :type "Array of /Game/Blueprints/AI/ChessFigure/BP_AIChessFigureBase Object Reference") (LDifferenceSignAndNumberInPosition :type Integer))
  (bind _array (`|MakeArray` "a" "b" "c" "d" "e" "f" "g" "h"))
  (bind _array_2 (`|MakeArray` "a" "b" "c" "d" "e" "f" "g" "h"))
  (bind _returnvalue (`KismetStringLibrary.Conv_StringToInt` (`KismetStringLibrary.GetSubstring` (`KismetStringLibrary.Conv_NameToString` (`local.LPositionCell`)) 1)))
  (bind _returnvalue_2 (`KismetStringLibrary.Conv_StringToInt` (`KismetStringLibrary.GetSubstring` (`KismetStringLibrary.Conv_NameToString` (`local.LPositionCell`)) 1)))
  (bind _returnvalue_3 (- 8 (`KismetStringLibrary.Conv_StringToInt` (`KismetStringLibrary.GetSubstring` (`KismetStringLibrary.Conv_NameToString` (`local.LPositionCell`)) 1))))
  (bind _returnvalue_4 (- 8 (`KismetStringLibrary.Conv_StringToInt` (`KismetStringLibrary.GetSubstring` (`KismetStringLibrary.Conv_NameToString` (`local.LPositionCell`)) 1))))
  (bind _returnvalue_5 (+ (`KismetArrayLibrary.Array_Find` (`|MakeArray` "h" "g" "f" "e" "d" "c" "b" "a") (`KismetStringLibrary.GetSubstring` (`KismetStringLibrary.Conv_NameToString` (`local.LPositionCell`)))) 1))
  (bind _returnvalue_6 (+ (`KismetArrayLibrary.Array_Find` (`|MakeArray` "a" "b" "c" "d" "e" "f" "g" "h") (`KismetStringLibrary.GetSubstring` (`KismetStringLibrary.Conv_NameToString` (`local.LPositionCell`)))) 1))
  (bind _returnvalue_7 (+ (`KismetArrayLibrary.Array_Find` (`|MakeArray` "a" "b" "c" "d" "e" "f" "g" "h") (`KismetStringLibrary.GetSubstring` (`KismetStringLibrary.Conv_NameToString` (`local.LPositionCell`)))) 1))
  (bind _returnvalue_8 (- 8 _returnvalue_5))
  (bind _returnvalue_9 (- 8 _returnvalue_7))
  (bind _returnvalue_10 (- 9 (+ (`KismetArrayLibrary.Array_Find` (`|MakeArray` "a" "b" "c" "d" "e" "f" "g" "h") (`KismetStringLibrary.GetSubstring` (`KismetStringLibrary.Conv_NameToString` (`local.LPositionCell`)))) 1)))
  (set `local.LPositionCell` (`|GetArrayItem` (`Actor.Tags` (`|GetArrayItem` (`self.GetOverlappingActors` "/Game/Blueprints/BattleField/BP_Cell.BP_Cell_C")))))
  (for _index (range 8)
    (switch `int` _index
      (:`0`
        ;[1 1 1] Up
        (for _index_2 (range (`KismetStringLibrary.Conv_StringToInt` (`KismetStringLibrary.GetSubstring` (`KismetStringLibrary.Conv_NameToString` (`local.LPositionCell`)) 1)) 9)
          (bind _returnvalue_11 (`KismetStringLibrary.Conv_StringToName` (`KismetStringLibrary.Concat_StrStr` (`KismetStringLibrary.GetSubstring` (`KismetStringLibrary.Conv_NameToString` (`local.LPositionCell`))) (`KismetStringLibrary.Conv_IntToString` _index_2))))
          (`KismetArrayLibrary.Array_AddUnique` (`self.AvailableMoves`) _returnvalue_11)
          (`self.CalculateCheck/FindFigureForDisable` _returnvalue_11 (`local.LPositionCell`) (`local.LDisableFigure`) true (`local.Attacker`) (`local.CellsOfAttacker`) (`local.CellsRemoveThreat`)))
        (`self.DisableFigure` (`local.LDisableFigure`))
        (`self.Check Cells Remove Threat` (`local.Attacker`) (`local.CellsRemoveThreat`)))
      (:`1`
        ;[1 1 1] Up-Right
        (`/Engine/EditorBlueprintResources/StandardMacros.CompareInt` _returnvalue_3 _returnvalue_9
          (:`>`
            (set `local.LDifferenceSignAndNumberInPosition` (- _returnvalue_3 _returnvalue_9))
            (for _index_3 (range _returnvalue_7 9)
              (bind _returnvalue_12 (`KismetStringLibrary.Conv_StringToName` (`KismetStringLibrary.Concat_StrStr` (`KismetStringLibrary.GetSubstring` (`|GetArrayItem` (`|MakeArray` "a" "b" "c" "d" "e" "f" "g" "h") (- _index_3 1))) (`KismetStringLibrary.Conv_IntToString` (- _index_3 (`local.LDifferenceSignAndNumberInPosition`))))))
              (`KismetArrayLibrary.Array_AddUnique` (`self.AvailableMoves`) _returnvalue_12)
              (`self.CalculateCheck/FindFigureForDisable` _returnvalue_12 (`local.LPositionCell`) (`local.LDisableFigure`) true (`local.Attacker`) (`local.CellsOfAttacker`) (`local.CellsRemoveThreat`)))
            (`self.DisableFigure` (`local.LDisableFigure`)))
          (:`==`
            (set `local.LDifferenceSignAndNumberInPosition` (- _returnvalue_9 _returnvalue_3) :!label _label)
            (for _index_4 (range (`KismetStringLibrary.Conv_StringToInt` (`KismetStringLibrary.GetSubstring` (`KismetStringLibrary.Conv_NameToString` (`local.LPositionCell`)) 1)) 9)
              (bind _returnvalue_13 (`KismetStringLibrary.Conv_StringToName` (`KismetStringLibrary.Concat_StrStr` (`KismetStringLibrary.GetSubstring` (`|GetArrayItem` (`|MakeArray` "a" "b" "c" "d" "e" "f" "g" "h") (- (- _index_4 (`local.LDifferenceSignAndNumberInPosition`)) 1))) (`KismetStringLibrary.Conv_IntToString` _index_4))))
              (`KismetArrayLibrary.Array_AddUnique` (`self.AvailableMoves`) _returnvalue_13)
              (`KismetSystemLibrary.PrintString` "Hello")
              (`self.CalculateCheck/FindFigureForDisable` _returnvalue_13 (`local.LPositionCell`) (`local.LDisableFigure`) true (`local.Attacker`) (`local.CellsOfAttacker`) (`local.CellsRemoveThreat`)))
            (`self.DisableFigure` (`local.LDisableFigure`))
            (`self.Check Cells Remove Threat` (`local.Attacker`) (`local.CellsRemoveThreat`)))
          (:`<`
            (goto _label))))
      (:`2`
        ;[1 1 1] Right
        (for _index_5 (range (`KismetArrayLibrary.Array_Find` (`|MakeArray` "a" "b" "c" "d" "e" "f" "g" "h") (`KismetStringLibrary.GetSubstring` (`KismetStringLibrary.Conv_NameToString` (`local.LPositionCell`)))) 8)
          (bind _returnvalue_14 (`KismetStringLibrary.Conv_StringToName` (`KismetStringLibrary.Concat_StrStr` (`|GetArrayItem` (`|MakeArray` "a" "b" "c" "d" "e" "f" "g" "h") _index_5) (`KismetStringLibrary.GetSubstring` (`KismetStringLibrary.Conv_NameToString` (`local.LPositionCell`)) 1))))
          (`KismetArrayLibrary.Array_AddUnique` (`self.AvailableMoves`) _returnvalue_14)
          (`self.CalculateCheck/FindFigureForDisable` _returnvalue_14 (`local.LPositionCell`) (`local.LDisableFigure`) true (`local.Attacker`) (`local.CellsOfAttacker`) (`local.CellsRemoveThreat`)))
        (`self.DisableFigure` (`local.LDisableFigure`))
        (`self.Check Cells Remove Threat` (`local.Attacker`) (`local.CellsRemoveThreat`)))
      (:`3`
        ;[1 1 1] Right-Down
        (`/Engine/EditorBlueprintResources/StandardMacros.CompareInt` _returnvalue_2 _returnvalue_10
          (:`>`
            (set `local.LDifferenceSignAndNumberInPosition` (- _returnvalue_2 _returnvalue_10))
            (for _index_6 (range (* _returnvalue_10 -1) 0)
              (bind _returnvalue_15 (* _index_6 -1))
              (bind _returnvalue_16 (`KismetStringLibrary.Conv_StringToName` (`KismetStringLibrary.Concat_StrStr` (`KismetStringLibrary.GetSubstring` (`|GetArrayItem` _array (- (+ (`KismetArrayLibrary.Array_LastIndex` _array) 1) _returnvalue_15))) (`KismetStringLibrary.Conv_IntToString` (+ _returnvalue_15 (`local.LDifferenceSignAndNumberInPosition`))))))
              (`KismetArrayLibrary.Array_AddUnique` (`self.AvailableMoves`) _returnvalue_16)
              (`self.CalculateCheck/FindFigureForDisable` _returnvalue_16 (`local.LPositionCell`) (`local.LDisableFigure`) true (`local.Attacker`) (`local.CellsOfAttacker`) (`local.CellsRemoveThreat`)))
            (`self.DisableFigure` (`local.LDisableFigure`))
            (`self.Check Cells Remove Threat` (`local.Attacker`) (`local.CellsRemoveThreat`)))
          (:`==`
            (set `local.LDifferenceSignAndNumberInPosition` (- _returnvalue_10 _returnvalue_2) :!label _label_2)
            (for _index_7 (range (* (`KismetStringLibrary.Conv_StringToInt` (`KismetStringLibrary.GetSubstring` (`KismetStringLibrary.Conv_NameToString` (`local.LPositionCell`)) 1)) -1) 0)
              (bind _returnvalue_17 (* _index_7 -1))
              (bind _returnvalue_18 (`KismetStringLibrary.Conv_StringToName` (`KismetStringLibrary.Concat_StrStr` (`KismetStringLibrary.GetSubstring` (`|GetArrayItem` _array_2 (- (+ (`KismetArrayLibrary.Array_LastIndex` _array_2) 1) (+ _returnvalue_17 (`local.LDifferenceSignAndNumberInPosition`))))) (`KismetStringLibrary.Conv_IntToString` _returnvalue_17))))
              (`KismetArrayLibrary.Array_AddUnique` (`self.AvailableMoves`) _returnvalue_18)
              (`self.CalculateCheck/FindFigureForDisable` _returnvalue_18 (`local.LPositionCell`) (`local.LDisableFigure`) true (`local.Attacker`) (`local.CellsOfAttacker`) (`local.CellsRemoveThreat`)))
            (`self.DisableFigure` (`local.LDisableFigure`))
            (`self.Check Cells Remove Threat` (`local.Attacker`) (`local.CellsRemoveThreat`)))
          (:`<`
            (goto _label_2))))
      (:`4`
        ;[1 1 1] Down
        (for _index_8 (range (* (`KismetStringLibrary.Conv_StringToInt` (`KismetStringLibrary.GetSubstring` (`KismetStringLibrary.Conv_NameToString` (`local.LPositionCell`)) 1)) -1) 0)
          (bind _returnvalue_19 (`KismetStringLibrary.Conv_StringToName` (`KismetStringLibrary.Concat_StrStr` (`KismetStringLibrary.GetSubstring` (`KismetStringLibrary.Conv_NameToString` (`local.LPositionCell`))) (`KismetStringLibrary.Conv_IntToString` (* _index_8 -1)))))
          (`KismetArrayLibrary.Array_AddUnique` (`self.AvailableMoves`) _returnvalue_19)
          (`self.CalculateCheck/FindFigureForDisable` _returnvalue_19 (`local.LPositionCell`) (`local.LDisableFigure`) true (`local.Attacker`) (`local.CellsOfAttacker`) (`local.CellsRemoveThreat`)))
        (`self.DisableFigure` (`local.LDisableFigure`))
        (`self.Check Cells Remove Threat` (`local.Attacker`) (`local.CellsRemoveThreat`)))
      (:`5`
        ;[1 1 1] Left-Down
        (`/Engine/EditorBlueprintResources/StandardMacros.CompareInt` _returnvalue _returnvalue_6
          (:`>`
            (set `local.LDifferenceSignAndNumberInPosition` (- _returnvalue _returnvalue_6))
            (for _index_9 (range (* _returnvalue_6 -1) 0)
              (bind _returnvalue_20 (* _index_9 -1))
              (bind _returnvalue_21 (`KismetStringLibrary.Conv_StringToName` (`KismetStringLibrary.Concat_StrStr` (`KismetStringLibrary.GetSubstring` (`|GetArrayItem` (`|MakeArray` "a" "b" "c" "d" "e" "f" "g" "h") (- _returnvalue_20 1))) (`KismetStringLibrary.Conv_IntToString` (+ _returnvalue_20 (`local.LDifferenceSignAndNumberInPosition`))))))
              (`KismetArrayLibrary.Array_AddUnique` (`self.AvailableMoves`) _returnvalue_21)
              (`self.CalculateCheck/FindFigureForDisable` _returnvalue_21 (`local.LPositionCell`) (`local.LDisableFigure`) true (`local.Attacker`) (`local.CellsOfAttacker`) (`local.CellsRemoveThreat`)))
            (`self.DisableFigure` (`local.LDisableFigure`))
            (`self.Check Cells Remove Threat` (`local.Attacker`) (`local.CellsRemoveThreat`)))
          (:`==`
            (set `local.LDifferenceSignAndNumberInPosition` (- _returnvalue_6 _returnvalue) :!label _label_3)
            (for _index_10 (range (* (`KismetStringLibrary.Conv_StringToInt` (`KismetStringLibrary.GetSubstring` (`KismetStringLibrary.Conv_NameToString` (`local.LPositionCell`)) 1)) -1) 0)
              (bind _returnvalue_22 (* _index_10 -1))
              (bind _returnvalue_23 (`KismetStringLibrary.Conv_StringToName` (`KismetStringLibrary.Concat_StrStr` (`KismetStringLibrary.GetSubstring` (`|GetArrayItem` (`|MakeArray` "a" "b" "c" "d" "e" "f" "g" "h") (- (+ _returnvalue_22 (`local.LDifferenceSignAndNumberInPosition`)) 1))) (`KismetStringLibrary.Conv_IntToString` _returnvalue_22))))
              (`KismetArrayLibrary.Array_AddUnique` (`self.AvailableMoves`) _returnvalue_23)
              (`self.CalculateCheck/FindFigureForDisable` _returnvalue_23 (`local.LPositionCell`) (`local.LDisableFigure`) true (`local.Attacker`) (`local.CellsOfAttacker`) (`local.CellsRemoveThreat`)))
            (`self.DisableFigure` (`local.LDisableFigure`))
            (`self.Check Cells Remove Threat` (`local.Attacker`) (`local.CellsRemoveThreat`)))
          (:`<`
            (goto _label_3))))
      (:`6`
        ;[1 1 1] Left
        (for _index_11 (range (`KismetArrayLibrary.Array_Find` (`|MakeArray` "h" "g" "f" "e" "d" "c" "b" "a") (`KismetStringLibrary.GetSubstring` (`KismetStringLibrary.Conv_NameToString` (`local.LPositionCell`)))) 8)
          (bind _returnvalue_24 (`KismetStringLibrary.Conv_StringToName` (`KismetStringLibrary.Concat_StrStr` (`|GetArrayItem` (`|MakeArray` "h" "g" "f" "e" "d" "c" "b" "a") _index_11) (`KismetStringLibrary.GetSubstring` (`KismetStringLibrary.Conv_NameToString` (`local.LPositionCell`)) 1))))
          (`KismetArrayLibrary.Array_AddUnique` (`self.AvailableMoves`) _returnvalue_24)
          (`self.CalculateCheck/FindFigureForDisable` _returnvalue_24 (`local.LPositionCell`) (`local.LDisableFigure`) true (`local.Attacker`) (`local.CellsOfAttacker`) (`local.CellsRemoveThreat`)))
        (`self.DisableFigure` (`local.LDisableFigure`))
        (`self.Check Cells Remove Threat` (`local.Attacker`) (`local.CellsRemoveThreat`)))
      (:`7`
        ;[1 1 1] Up-Left
        (`/Engine/EditorBlueprintResources/StandardMacros.CompareInt` _returnvalue_4 _returnvalue_8
          (:`>`
            (set `local.LDifferenceSignAndNumberInPosition` (- _returnvalue_4 _returnvalue_8))
            (for _index_12 (range _returnvalue_5 9)
              (bind _returnvalue_25 (`KismetStringLibrary.Conv_StringToName` (`KismetStringLibrary.Concat_StrStr` (`KismetStringLibrary.GetSubstring` (`|GetArrayItem` (`|MakeArray` "h" "g" "f" "e" "d" "c" "b" "a") (- _index_12 1))) (`KismetStringLibrary.Conv_IntToString` (- _index_12 (`local.LDifferenceSignAndNumberInPosition`))))))
              (`KismetArrayLibrary.Array_AddUnique` (`self.AvailableMoves`) _returnvalue_25)
              (`self.CalculateCheck/FindFigureForDisable` _returnvalue_25 (`local.LPositionCell`) (`local.LDisableFigure`) true (`local.Attacker`) (`local.CellsOfAttacker`) (`local.CellsRemoveThreat`)))
            (`self.DisableFigure` (`local.LDisableFigure`))
            (`self.Check Cells Remove Threat` (`local.Attacker`) (`local.CellsRemoveThreat`)))
          (:`==`
            (set `local.LDifferenceSignAndNumberInPosition` (- _returnvalue_8 _returnvalue_4) :!label _label_4)
            (for _index_13 (range (`KismetStringLibrary.Conv_StringToInt` (`KismetStringLibrary.GetSubstring` (`KismetStringLibrary.Conv_NameToString` (`local.LPositionCell`)) 1)) 9)
              (bind _returnvalue_26 (`KismetStringLibrary.Conv_StringToName` (`KismetStringLibrary.Concat_StrStr` (`KismetStringLibrary.GetSubstring` (`|GetArrayItem` (`|MakeArray` "h" "g" "f" "e" "d" "c" "b" "a") (- (- _index_13 (`local.LDifferenceSignAndNumberInPosition`)) 1))) (`KismetStringLibrary.Conv_IntToString` _index_13))))
              (`KismetArrayLibrary.Array_AddUnique` (`self.AvailableMoves`) _returnvalue_26)
              (`self.CalculateCheck/FindFigureForDisable` _returnvalue_26 (`local.LPositionCell`) (`local.LDisableFigure`) true (`local.Attacker`) (`local.CellsOfAttacker`) (`local.CellsRemoveThreat`)))
            (`self.DisableFigure` (`local.LDisableFigure`))
            (`self.Check Cells Remove Threat` (`local.Attacker`) (`local.CellsRemoveThreat`)))
          (:`<`
            (goto _label_4)))))))

(fn `UserConstructionScript`
  (`parent.UserConstructionScript`))