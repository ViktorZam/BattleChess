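; Pawn chess piece that sets its promotion rank from its starting cell and works out where it can step or capture.
; SpawnPawnGrid spawns a temporary box-collision grid, shows valid steps using box tags (move, fight, first step) and cell occupancy, then destroys it.
; For check calculation, CalculateStepsPawn derives forward, diagonal and first double-step cells from algebraic cell tags and facing, feeding figure-disable and threat-removal checks.
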(event `self.ReceiveBeginPlay`
  (`parent.ReceiveBeginPlay`)
  (if (!= (`KismetArrayLibrary.Array_Length` (`self.GetOverlappingActors` "/Game/Blueprints/BattleField/BP_Cell.BP_Cell_C")) 0)
    (switch `string` (`KismetStringLibrary.GetSubstring` (`KismetStringLibrary.Conv_NameToString` (`|GetArrayItem` (`Actor.Tags` (`|GetArrayItem` (`self.GetOverlappingActors` "/Game/Blueprints/BattleField/BP_Cell.BP_Cell_C"))))) 1)
      (:`2`
        (set `self.NumberCellsForUpgrade` 8))
      (:`7`
        (set `self.NumberCellsForUpgrade` 1)))))

(event `/Game/Blueprints/Interfaces/BPI_Figures.SetGridSteps`
  (`self.Spawn Pawn Grid`))

(event `/Game/Blueprints/Interfaces/BPI_Figures.CalculateCheck/DisableFigures`
  (params (Attacker :type "/Game/Blueprints/AI/ChessFigure/BP_AIChessFigureBase Object Reference") (CellsOfAttacker :type "Array of Name (by ref)") (CellsRemoveThreat :type "Array of String (by ref)"))
  ;[1 1 1] Find figure for disable
  (`self.CalculateStepsPawn` Attacker CellsOfAttacker CellsRemoveThreat))

(event `/Game/Blueprints/Interfaces/BPI_Figures.SetUsedFirstStep`
  (`/Engine/EditorBlueprintResources/StandardMacros.DoOnce` false
    (:`Completed`
      (set `self.FirstStepUsed?` true))))

(event `self.ReceiveTick`
  (params (DeltaSeconds :type "Float (single-precision)")))

(fn `CalculateStepsPawn`
  (params (Attacker :type "/Game/Blueprints/AI/ChessFigure/BP_AIChessFigureBase Object Reference") (CellsOfAttacker :type "Array of Name (by ref)") (CellsRemoveThreat :type "Array of String (by ref)"))
  (locals (LPositionCell :type Name) (LDisableFigure :type "Array of /Game/Blueprints/AI/ChessFigure/BP_AIChessFigureBase Object Reference") (LDifferenceSignAndNumberInPosition :type Integer))
  (bind _returnvalue (`KismetStringLibrary.Conv_StringToName` (`KismetStringLibrary.Concat_StrStr` (`|GetArrayItem` (`|MakeArray` "a" "b" "c" "d" "e" "f" "g" "h") (- (`KismetArrayLibrary.Array_Find` (`|MakeArray` "a" "b" "c" "d" "e" "f" "g" "h") (`KismetStringLibrary.GetSubstring` (`KismetStringLibrary.Conv_NameToString` (`local.LPositionCell`)))) 1)) (`KismetStringLibrary.Conv_IntToString` (+ (`KismetStringLibrary.Conv_StringToInt` (`KismetStringLibrary.GetSubstring` (`KismetStringLibrary.Conv_NameToString` (`local.LPositionCell`)) 1)) 1)))))
  (bind _returnvalue_2 (`KismetStringLibrary.Conv_StringToName` (`KismetStringLibrary.Concat_StrStr` (`|GetArrayItem` (`|MakeArray` "a" "b" "c" "d" "e" "f" "g" "h") (+ (`KismetArrayLibrary.Array_Find` (`|MakeArray` "a" "b" "c" "d" "e" "f" "g" "h") (`KismetStringLibrary.GetSubstring` (`KismetStringLibrary.Conv_NameToString` (`local.LPositionCell`)))) 1)) (`KismetStringLibrary.Conv_IntToString` (- (`KismetStringLibrary.Conv_StringToInt` (`KismetStringLibrary.GetSubstring` (`KismetStringLibrary.Conv_NameToString` (`local.LPositionCell`)) 1)) 1)))))
  (bind _returnvalue_3 (`KismetStringLibrary.Conv_StringToName` (`KismetStringLibrary.Concat_StrStr` (`|GetArrayItem` (`|MakeArray` "a" "b" "c" "d" "e" "f" "g" "h") (`KismetArrayLibrary.Array_Find` (`|MakeArray` "a" "b" "c" "d" "e" "f" "g" "h") (`KismetStringLibrary.GetSubstring` (`KismetStringLibrary.Conv_NameToString` (`local.LPositionCell`))))) (`KismetStringLibrary.Conv_IntToString` (+ (`KismetStringLibrary.Conv_StringToInt` (`KismetStringLibrary.GetSubstring` (`KismetStringLibrary.Conv_NameToString` (`local.LPositionCell`)) 1)) 1)))))
  (bind _returnvalue_4 (`KismetStringLibrary.Conv_StringToName` (`KismetStringLibrary.Concat_StrStr` (`|GetArrayItem` (`|MakeArray` "a" "b" "c" "d" "e" "f" "g" "h") (`KismetArrayLibrary.Array_Find` (`|MakeArray` "a" "b" "c" "d" "e" "f" "g" "h") (`KismetStringLibrary.GetSubstring` (`KismetStringLibrary.Conv_NameToString` (`local.LPositionCell`))))) (`KismetStringLibrary.Conv_IntToString` (- (`KismetStringLibrary.Conv_StringToInt` (`KismetStringLibrary.GetSubstring` (`KismetStringLibrary.Conv_NameToString` (`local.LPositionCell`)) 1)) 1)))))
  (bind _returnvalue_5 (`KismetStringLibrary.Conv_StringToName` (`KismetStringLibrary.Concat_StrStr` (`|GetArrayItem` (`|MakeArray` "a" "b" "c" "d" "e" "f" "g" "h") (`KismetArrayLibrary.Array_Find` (`|MakeArray` "a" "b" "c" "d" "e" "f" "g" "h") (`KismetStringLibrary.GetSubstring` (`KismetStringLibrary.Conv_NameToString` (`local.LPositionCell`))))) (`KismetStringLibrary.Conv_IntToString` (- (`KismetStringLibrary.Conv_StringToInt` (`KismetStringLibrary.GetSubstring` (`KismetStringLibrary.Conv_NameToString` (`local.LPositionCell`)) 1)) 2)))))
  (bind _returnvalue_6 (`KismetStringLibrary.Conv_StringToName` (`KismetStringLibrary.Concat_StrStr` (`|GetArrayItem` (`|MakeArray` "a" "b" "c" "d" "e" "f" "g" "h") (`KismetArrayLibrary.Array_Find` (`|MakeArray` "a" "b" "c" "d" "e" "f" "g" "h") (`KismetStringLibrary.GetSubstring` (`KismetStringLibrary.Conv_NameToString` (`local.LPositionCell`))))) (`KismetStringLibrary.Conv_IntToString` (+ (`KismetStringLibrary.Conv_StringToInt` (`KismetStringLibrary.GetSubstring` (`KismetStringLibrary.Conv_NameToString` (`local.LPositionCell`)) 1)) 2)))))
  (bind _returnvalue_7 (`KismetStringLibrary.Conv_StringToName` (`KismetStringLibrary.Concat_StrStr` (`|GetArrayItem` (`|MakeArray` "a" "b" "c" "d" "e" "f" "g" "h") (+ (`KismetArrayLibrary.Array_Find` (`|MakeArray` "a" "b" "c" "d" "e" "f" "g" "h") (`KismetStringLibrary.GetSubstring` (`KismetStringLibrary.Conv_NameToString` (`local.LPositionCell`)))) 1)) (`KismetStringLibrary.Conv_IntToString` (+ (`KismetStringLibrary.Conv_StringToInt` (`KismetStringLibrary.GetSubstring` (`KismetStringLibrary.Conv_NameToString` (`local.LPositionCell`)) 1)) 1)))))
  (bind _returnvalue_8 (`KismetStringLibrary.Conv_StringToName` (`KismetStringLibrary.Concat_StrStr` (`|GetArrayItem` (`|MakeArray` "a" "b" "c" "d" "e" "f" "g" "h") (- (`KismetArrayLibrary.Array_Find` (`|MakeArray` "a" "b" "c" "d" "e" "f" "g" "h") (`KismetStringLibrary.GetSubstring` (`KismetStringLibrary.Conv_NameToString` (`local.LPositionCell`)))) 1)) (`KismetStringLibrary.Conv_IntToString` (- (`KismetStringLibrary.Conv_StringToInt` (`KismetStringLibrary.GetSubstring` (`KismetStringLibrary.Conv_NameToString` (`local.LPositionCell`)) 1)) 1)))))
  (set `local.LPositionCell` (`|GetArrayItem` (`Actor.Tags` (`|GetArrayItem` (`self.GetOverlappingActors` "/Game/Blueprints/BattleField/BP_Cell.BP_Cell_C")))))
  (for _index (range 3)
    (switch `int` _index
      (:`0`
        ;[1 1 1] Left-Up
        (if (`KismetMathLibrary.NearlyEqual_FloatFloat` (`KismetMathLibrary.Abs` (`self.DefaultZRotation`)) 0.0 1.0)
          (`/Engine/EditorBlueprintResources/StandardMacros.CompareInt` (+ (`KismetStringLibrary.Conv_StringToInt` (`KismetStringLibrary.GetSubstring` (`KismetStringLibrary.Conv_NameToString` (`local.LPositionCell`)) 1)) 1) 8
            (:`==`
              _)
            (:`<`
              _))
          (`/Engine/EditorBlueprintResources/StandardMacros.CompareInt` (- (`KismetArrayLibrary.Array_Find` (`|MakeArray` "a" "b" "c" "d" "e" "f" "g" "h") (`KismetStringLibrary.GetSubstring` (`KismetStringLibrary.Conv_NameToString` (`local.LPositionCell`)))) 1)
            (:`>`
              _)
            (:`==`
              _))
          (`KismetArrayLibrary.Array_AddUnique` (`self.AvailableMoves`) _returnvalue)
          (`self.CalculateCheck/FindFigureForDisable` _returnvalue (`local.LPositionCell`) (`local.LDisableFigure`) true (`local.Attacker`) (`local.CellsOfAttacker`) (`local.CellsRemoveThreat`))
          (`self.Check Cells Remove Threat` (`local.Attacker`) (`local.CellsRemoveThreat`))
          (else
            (`/Engine/EditorBlueprintResources/StandardMacros.CompareInt` (- (`KismetStringLibrary.Conv_StringToInt` (`KismetStringLibrary.GetSubstring` (`KismetStringLibrary.Conv_NameToString` (`local.LPositionCell`)) 1)) 1)
              (:`>`
                _)
              (:`==`
                _))
            (`/Engine/EditorBlueprintResources/StandardMacros.CompareInt` (+ (`KismetArrayLibrary.Array_Find` (`|MakeArray` "a" "b" "c" "d" "e" "f" "g" "h") (`KismetStringLibrary.GetSubstring` (`KismetStringLibrary.Conv_NameToString` (`local.LPositionCell`)))) 1) 7
              (:`==`
                _)
              (:`<`
                _))
            (`KismetArrayLibrary.Array_AddUnique` (`self.AvailableMoves`) _returnvalue_2)
            (`self.CalculateCheck/FindFigureForDisable` _returnvalue_2 (`local.LPositionCell`) (`local.LDisableFigure`) true (`local.Attacker`) (`local.CellsOfAttacker`) (`local.CellsRemoveThreat`))
            (`self.Check Cells Remove Threat` (`local.Attacker`) (`local.CellsRemoveThreat`)))))
      (:`1`
        ;[1 1 1] Up
        (if (`KismetMathLibrary.NearlyEqual_FloatFloat` (`KismetMathLibrary.Abs` (`self.DefaultZRotation`)) 0.0 1.0)
          (`/Engine/EditorBlueprintResources/StandardMacros.CompareInt` (+ (`KismetStringLibrary.Conv_StringToInt` (`KismetStringLibrary.GetSubstring` (`KismetStringLibrary.Conv_NameToString` (`local.LPositionCell`)) 1)) 1) 8
            (:`==`
              _)
            (:`<`
              _))
          (`KismetArrayLibrary.Array_AddUnique` (`self.AvailableMoves`) _returnvalue_3)
          (`self.CalculateCheck/FindFigureForDisable` _returnvalue_3 (`local.LPositionCell`) (`local.LDisableFigure`) false (`local.Attacker`) (`local.CellsOfAttacker`) (`local.CellsRemoveThreat`))
          (`self.Check Cells Remove Threat` (`local.Attacker`) (`local.CellsRemoveThreat`))
          (else
            (`/Engine/EditorBlueprintResources/StandardMacros.CompareInt` (- (`KismetStringLibrary.Conv_StringToInt` (`KismetStringLibrary.GetSubstring` (`KismetStringLibrary.Conv_NameToString` (`local.LPositionCell`)) 1)) 1)
              (:`>`
                _)
              (:`==`
                _))
            (`KismetArrayLibrary.Array_AddUnique` (`self.AvailableMoves`) _returnvalue_4)
            (`self.CalculateCheck/FindFigureForDisable` _returnvalue_4 (`local.LPositionCell`) (`local.LDisableFigure`) false (`local.Attacker`) (`local.CellsOfAttacker`) (`local.CellsRemoveThreat`))
            (`self.Check Cells Remove Threat` (`local.Attacker`) (`local.CellsRemoveThreat`)))))
      (:`2`
        ;[1 1 1] Right-Up
        (if (`KismetMathLibrary.NearlyEqual_FloatFloat` (`KismetMathLibrary.Abs` (`self.DefaultZRotation`)) 0.0 1.0)
          (`/Engine/EditorBlueprintResources/StandardMacros.CompareInt` (+ (`KismetStringLibrary.Conv_StringToInt` (`KismetStringLibrary.GetSubstring` (`KismetStringLibrary.Conv_NameToString` (`local.LPositionCell`)) 1)) 1) 8
            (:`==`
              _)
            (:`<`
              _))
          (`/Engine/EditorBlueprintResources/StandardMacros.CompareInt` (+ (`KismetArrayLibrary.Array_Find` (`|MakeArray` "a" "b" "c" "d" "e" "f" "g" "h") (`KismetStringLibrary.GetSubstring` (`KismetStringLibrary.Conv_NameToString` (`local.LPositionCell`)))) 1) 7
            (:`==`
              _)
            (:`<`
              _))
          (`KismetArrayLibrary.Array_AddUnique` (`self.AvailableMoves`) _returnvalue_7)
          (`self.CalculateCheck/FindFigureForDisable` _returnvalue_7 (`local.LPositionCell`) (`local.LDisableFigure`) true (`local.Attacker`) (`local.CellsOfAttacker`) (`local.CellsRemoveThreat`))
          (`self.Check Cells Remove Threat` (`local.Attacker`) (`local.CellsRemoveThreat`))
          (else
            (`/Engine/EditorBlueprintResources/StandardMacros.CompareInt` (- (`KismetStringLibrary.Conv_StringToInt` (`KismetStringLibrary.GetSubstring` (`KismetStringLibrary.Conv_NameToString` (`local.LPositionCell`)) 1)) 1)
              (:`>`
                _)
              (:`==`
                _))
            (`/Engine/EditorBlueprintResources/StandardMacros.CompareInt` (- (`KismetArrayLibrary.Array_Find` (`|MakeArray` "a" "b" "c" "d" "e" "f" "g" "h") (`KismetStringLibrary.GetSubstring` (`KismetStringLibrary.Conv_NameToString` (`local.LPositionCell`)))) 1)
              (:`>`
                _)
              (:`==`
                _))
            (`KismetArrayLibrary.Array_AddUnique` (`self.AvailableMoves`) _returnvalue_8)
            (`self.CalculateCheck/FindFigureForDisable` _returnvalue_8 (`local.LPositionCell`) (`local.LDisableFigure`) true (`local.Attacker`) (`local.CellsOfAttacker`) (`local.CellsRemoveThreat`))
            (`self.Check Cells Remove Threat` (`local.Attacker`) (`local.CellsRemoveThreat`)))))))
  (if (not (`self.FirstStepUsed?`))
    ;[1 1 1] Up
    (if (`KismetMathLibrary.NearlyEqual_FloatFloat` (`KismetMathLibrary.Abs` (`self.DefaultZRotation`)) 0.0 1.0)
      (`/Engine/EditorBlueprintResources/StandardMacros.CompareInt` (+ (`KismetStringLibrary.Conv_StringToInt` (`KismetStringLibrary.GetSubstring` (`KismetStringLibrary.Conv_NameToString` (`local.LPositionCell`)) 1)) 2) 8
        (:`==`
          _)
        (:`<`
          _))
      (`KismetArrayLibrary.Array_AddUnique` (`self.AvailableMoves`) _returnvalue_6)
      (`self.CalculateCheck/FindFigureForDisable` _returnvalue_6 (`local.LPositionCell`) (`local.LDisableFigure`) false (`local.Attacker`) (`local.CellsOfAttacker`) (`local.CellsRemoveThreat`))
      (`self.Check Cells Remove Threat` (`local.Attacker`) (`local.CellsRemoveThreat`))
      (else
        (`/Engine/EditorBlueprintResources/StandardMacros.CompareInt` (- (`KismetStringLibrary.Conv_StringToInt` (`KismetStringLibrary.GetSubstring` (`KismetStringLibrary.Conv_NameToString` (`local.LPositionCell`)) 1)) 2)
          (:`>`
            _)
          (:`==`
            _))
        (`KismetArrayLibrary.Array_AddUnique` (`self.AvailableMoves`) _returnvalue_5)
        (`self.CalculateCheck/FindFigureForDisable` _returnvalue_5 (`local.LPositionCell`) (`local.LDisableFigure`) false (`local.Attacker`) (`local.CellsOfAttacker`) (`local.CellsRemoveThreat`))
        (`self.Check Cells Remove Threat` (`local.Attacker`) (`local.CellsRemoveThreat`))))))

(fn `Spawn Pawn Grid`
  (locals (LGrid :type "Actor Object Reference") (LDestroyerComponents :type "/Game/Blueprints/BattleField/BP_DestroyerComponents Object Reference") (LBox :type "BoxComponent Object Reference") (LIndex :type Integer))
  (bind _overlappingactors (`self.GetOverlappingActors` "/Game/Blueprints/BattleField/BP_Cell.BP_Cell_C"))
  (bind (_returnvalue_roll _returnvalue_pitch _returnvalue_yaw) (`KismetMathLibrary.BreakRotator` (`self.K2_GetActorRotation`)))
  (bind _asbp_aichess_figure_base (cast `/Game/Blueprints/AI/ChessFigure/BP_AIChessFigureBase` (`|GetArrayItem` (`self.GetOverlappingActors` (`|GetArrayItem` (`PrimitiveComponent.GetOverlappingActors` (`local.LBox`) "/Game/Blueprints/BattleField/BP_Cell.BP_Cell_C")) "/Game/Blueprints/AI/ChessFigure/BP_AIChessFigureBase.BP_AIChessFigureBase_C")) :!pure true))
  (if (!= (`KismetArrayLibrary.Array_Length` _overlappingactors) 0)
    (bind _returnvalue (`|SpawnActorFromClass` (`self.GridType`) (`KismetMathLibrary.MakeTransform` (`self.K2_GetActorLocation` (`|GetArrayItem` _overlappingactors)) (`KismetMathLibrary.MakeRotator` 0.0 0.0 (`KismetMathLibrary.FClamp` (`KismetMathLibrary.ClampAxis` _returnvalue_yaw) 0.0 180.0))) "Undefined" "OverrideRootScale" null null))
    (set `local.LGrid` _returnvalue)
    (bind _returnvalue_2 (`|SpawnActorFromClass` "/Game/Blueprints/BattleField/BP_DestroyerComponents.BP_DestroyerComponents_C" (`KismetMathLibrary.MakeTransform` (0.0 0.0 1000.0)) "Undefined" "OverrideRootScale" null null))
    (set `local.LDestroyerComponents` _returnvalue_2)
    (for (_array_element _array_index) (`self.K2_GetComponentsByClass` (`local.LGrid`) "/Script/Engine.BoxComponent")
      (set `local.LBox` _array_element)
      (set `local.LIndex` _array_index)
      (if (== (`KismetArrayLibrary.Array_Length` (`PrimitiveComponent.GetOverlappingActors` (`local.LBox`) "/Game/Blueprints/BattleField/BP_Cell.BP_Cell_C")) 0)
        (`self.AttachBox CollisionToDestroyer` (`local.LBox`) (`local.LDestroyerComponents`) :!label _label)
        (elif (!= (`KismetArrayLibrary.Array_Length` (`ActorComponent.ComponentTags` (`local.LBox`))) 0)
          (switch `name` (`|GetArrayItem` (`ActorComponent.ComponentTags` (`local.LBox`)))
            (:`Default`
              (if (== (`KismetArrayLibrary.Array_Length` (`self.GetOverlappingActors` (`|GetArrayItem` (`PrimitiveComponent.GetOverlappingActors` (`local.LBox`) "/Game/Blueprints/BattleField/BP_Cell.BP_Cell_C")) "/Game/Blueprints/AI/ChessFigure/BP_AIChessFigureBase.BP_AIChessFigureBase_C")) 0) :!label _label_2
                (`self.AttachBox CollisionToDestroyer` (`local.LBox`) (`local.LDestroyerComponents`))
                (elif (== _asbp_aichess_figure_base self)
                  _
                  (elif (== (`|GetArrayItem` (`Actor.Tags` _asbp_aichess_figure_base)) (`|GetArrayItem` (`self.Tags`)))
                    (`self.AttachBox CollisionToDestroyer` (`local.LBox`) (`local.LDestroyerComponents`))
                    (else
                      (`self.ShowAvailableStep` (`local.LBox`))
                      (`self.AttachBox CollisionToDestroyer` (`local.LBox`) (`local.LDestroyerComponents`)))))))
            (:`OnlyFirstStep`
              (if (`self.FirstStepUsed?`)
                (goto _label)
                (else
                  (if (== (`KismetArrayLibrary.Array_Length` (`self.GetOverlappingActors` (`|GetArrayItem` (`PrimitiveComponent.GetOverlappingActors` (`local.LBox`) "/Game/Blueprints/BattleField/BP_Cell.BP_Cell_C")) "/Game/Blueprints/AI/ChessFigure/BP_AIChessFigureBase.BP_AIChessFigureBase_C")) 0) :!label _label_3
                    (`self.ShowAvailableStep` (`local.LBox`))
                    (else
                      (`self.AttachBox CollisionToDestroyer` (`local.LBox`) (`local.LDestroyerComponents`)))))))
            (:`OnlyMove`
              (goto _label_3))
            (:`OnlyFight`
              (goto _label_2))))))
    (`self.K2_DestroyActor` (`local.LGrid`))
    (`self.K2_DestroyActor` (`local.LDestroyerComponents`))))

(fn `UserConstructionScript`
  (`parent.UserConstructionScript`))