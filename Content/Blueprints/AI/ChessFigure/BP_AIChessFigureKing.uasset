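; AI-controlled chess king piece that computes its available moves, including castling, and repositions the rook when castling.
; Moves come from temporary grid actors whose box overlaps are tested against cells, pieces and a grid spawned on the enemy king, with invalid boxes attached to a destroyer actor.
; Castling boxes are dropped when blocked or the rook has moved.
; After its first step the king switches to the plain grid and, on a castling square, shifts the nearest rook.
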(event `self.ReceiveBeginPlay`
  (`parent.ReceiveBeginPlay`))

(event `/Game/Blueprints/Interfaces/BPI_Figures.SetGridSteps`
  (`self.SpawnKingGridSteps`))

(event `/Game/Blueprints/Interfaces/BPI_Figures.SetUsedFirstStep`
  (`/Engine/EditorBlueprintResources/StandardMacros.DoOnce` false
    (:`Completed`
      (`self.CastlingRook`))))

(fn `CastlingRook`
  (locals (LDistanceRookForCastling :type "Float (double-precision)" :default 10000.0) (LRook :type "Actor Object Reference") (LGrid :type "/Game/Blueprints/AI/GridsSteps/King/BP_GridCastling Object Reference"))
  (bind (_returnvalue_x _returnvalue_y _returnvalue_z) (`KismetMathLibrary.BreakVector` (`self.K2_GetActorLocation` (`local.LRook`))))
  (bind (_returnvalue_x_2 _returnvalue_y_2 _returnvalue_z_2) (`KismetMathLibrary.BreakVector` (`self.K2_GetActorLocation` (`local.LRook`))))
  (bind (_returnvalue_roll _returnvalue_pitch _returnvalue_yaw) (`KismetMathLibrary.BreakRotator` (`KismetMathLibrary.FindLookAtRotation` (`self.K2_GetActorLocation` (`local.LRook`)) (`self.K2_GetActorLocation`))))
  (bind (_returnvalue_x_3 _returnvalue_y_3) (`KismetMathLibrary.BreakVector` (`self.K2_GetActorLocation` (`|GetArrayItem` (`PrimitiveComponent.GetOverlappingActors` (`|GetArrayItem` (`self.GetComponentsByTag` (`local.LGrid`) "/Script/Engine.BoxComponent" "Left")) "/Game/Blueprints/BattleField/BP_Cell.BP_Cell_C")))))
  (bind (_returnvalue_x_4 _returnvalue_y_4) (`KismetMathLibrary.BreakVector` (`self.K2_GetActorLocation` (`|GetArrayItem` (`PrimitiveComponent.GetOverlappingActors` (`|GetArrayItem` (`self.GetComponentsByTag` (`local.LGrid`) "/Script/Engine.BoxComponent" "Right")) "/Game/Blueprints/BattleField/BP_Cell.BP_Cell_C")))))
  (set `self.GridType` "/Game/Blueprints/AI/GridsSteps/King/BP_GridStepsKing.BP_GridStepsKing_C")
  (switch `name` (`|GetArrayItem` (`Actor.Tags` (`|GetArrayItem` (`self.GetOverlappingActors` "/Game/Blueprints/BattleField/BP_Cell.BP_Cell_C"))))
    (:`c1`
      _)
    (:`g1`
      _)
    (:`c8`
      _)
    (:`g8`
      _))
  (bind _outactors (`GameplayStatics.GetAllActorsOfClassWithTag` "/Game/Blueprints/AI/ChessFigure/BP_AIChessFigureRook.BP_AIChessFigureRook_C" (`|GetArrayItem` (`self.Tags`))))
  (for _array_element _outactors
    (bind _returnvalue (`KismetMathLibrary.Vector_Distance` (`self.K2_GetActorLocation` _array_element) (`self.K2_GetActorLocation`)))
    (if (< _returnvalue (`local.LDistanceRookForCastling`))
      (set `local.LDistanceRookForCastling` _returnvalue)
      (set `local.LRook` _array_element)))
  (`self.SetActorHiddenInGame` (`local.LRook`) true)
  (bind _returnvalue_2 (`|SpawnActorFromClass` "/Game/Blueprints/AI/GridsSteps/King/BP_GridCastling.BP_GridCastling_C" (`KismetMathLibrary.MakeTransform` (`self.K2_GetActorLocation` (`|GetArrayItem` (`self.GetOverlappingActors` "/Game/Blueprints/BattleField/BP_Cell.BP_Cell_C")))) "Undefined" "OverrideRootScale" null null))
  (set `local.LGrid` _returnvalue_2)
  (if (> _returnvalue_yaw 0.0)
    (`self.K2_SetActorLocation` (`local.LRook`) (`KismetMathLibrary.MakeVector` _returnvalue_x_4 _returnvalue_y_4 _returnvalue_z_2) false false)
    (else
      (`self.K2_SetActorLocation` (`local.LRook`) (`KismetMathLibrary.MakeVector` _returnvalue_x_3 _returnvalue_y_3 _returnvalue_z) false false)))
  (`self.SetActorHiddenInGame` (`local.LRook`) false)
  (`self.K2_DestroyActor` (`local.LGrid`)))

(fn `HandlerAvailableStepsKing`
  (params (LBox :type "BoxComponent Object Reference") (DestroyerComponents :type "/Game/Blueprints/BattleField/BP_DestroyerComponents Object Reference"))
  (returns (`LDelLeftCastlingBoxOut?` :type Boolean) (`LDelRightCastlingBoxOut?` :type Boolean))
  (locals (`LDelLeftCastlingBox?` :type Boolean) (`LDelRightCastlingBox?` :type Boolean))
  (bind _output (`|GetArrayItem` (`ActorComponent.ComponentTags` (`local.LBox`))))
  (bind _overlappingactors (`self.GetOverlappingActors` (`|GetArrayItem` (`PrimitiveComponent.GetOverlappingActors` (`local.LBox`) "/Game/Blueprints/BattleField/BP_Cell.BP_Cell_C")) "/Game/Blueprints/AI/ChessFigure/BP_AIChessFigureBase.BP_AIChessFigureBase_C"))
  (bind _asbp_aichess_figure_base (cast `/Game/Blueprints/AI/ChessFigure/BP_AIChessFigureBase` (`|GetArrayItem` _overlappingactors) :!pure true))
  (if (== (`KismetArrayLibrary.Array_Length` (`PrimitiveComponent.GetOverlappingActors` (`local.LBox`) "/Game/Blueprints/BattleField/BP_Cell.BP_Cell_C")) 0)
    (`self.AttachBox CollisionToDestroyer` (`local.LBox`) (`local.DestroyerComponents`))
    (return (`local.LDelLeftCastlingBox?`) (`local.LDelRightCastlingBox?`))
    (elif (== (`KismetArrayLibrary.Array_Length` _overlappingactors) 0)
      (if (not (!= (`KismetArrayLibrary.Array_Length` (`ActorComponent.ComponentTags` (`local.LBox`))) 0))
        (`self.ShowAvailableStep` (`local.LBox`)))
      (return (`local.LDelLeftCastlingBox?`) (`local.LDelRightCastlingBox?`))
      (elif (== _asbp_aichess_figure_base self)
        (return (`local.LDelLeftCastlingBox?`) (`local.LDelRightCastlingBox?`))
        (elif (== (`|GetArrayItem` (`Actor.Tags` _asbp_aichess_figure_base)) (`|GetArrayItem` (`self.Tags`)))
          (`self.AttachBox CollisionToDestroyer` (`local.LBox`) (`local.DestroyerComponents`))
          (return (`local.LDelLeftCastlingBox?`) (`local.LDelRightCastlingBox?`))
          (else
            (if (!= (`KismetArrayLibrary.Array_Length` (`ActorComponent.ComponentTags` (`local.LBox`))) 0)
              (if (== _output "LeftCastling")
                (set `local.LDelLeftCastlingBox?` true)
                (elif (== _output "RightCastling")
                  (set `local.LDelRightCastlingBox?` true)
                  (else
                    (`self.ShowAvailableStep` (`local.LBox`) :!label _label))))
              (else
                (goto _label)))
            (`self.AttachBox CollisionToDestroyer` (`local.LBox`) (`local.DestroyerComponents`))
            (return (`local.LDelLeftCastlingBox?`) (`local.LDelRightCastlingBox?`))))))))

(fn `SpawnKingGridSteps`
  (locals (LGridSelfKing :type "Actor Object Reference") (LBox :type "BoxComponent Object Reference") (LIndex :type Integer) (LGridEnemyKing :type "/Game/Blueprints/AI/GridsSteps/King/BP_GridStepsKing Object Reference") (`LDelLeftCastlingBox?` :type Boolean :default false) (`LDelRightCastlingBox?` :type Boolean) (LGridFindRook :type "Object Object Reference") (LDestroyerComponents :type "/Game/Blueprints/BattleField/BP_DestroyerComponents Object Reference"))
  (bind _overlappingactors (`self.GetOverlappingActors` "/Game/Blueprints/BattleField/BP_Cell.BP_Cell_C"))
  (if (!= (`KismetArrayLibrary.Array_Length` _overlappingactors) 0)
    (bind _returnvalue (`|SpawnActorFromClass` (`self.GridType`) (`KismetMathLibrary.MakeTransform` (`self.K2_GetActorLocation` (`|GetArrayItem` _overlappingactors))) "Undefined" "OverrideRootScale" null null))
    (set `local.LGridSelfKing` _returnvalue)
    (bind _returnvalue_2 (`|SpawnActorFromClass` "/Game/Blueprints/BattleField/BP_DestroyerComponents.BP_DestroyerComponents_C" (`KismetMathLibrary.MakeTransform` (0.0 0.0 1000.0)) "Undefined" "OverrideRootScale" null null))
    (set `local.LDestroyerComponents` _returnvalue_2)
    (if (== (`|GetArrayItem` (`self.Tags`)) "White")
      (bind _outactors (`GameplayStatics.GetAllActorsOfClassWithTag` "BP_AIChessFigureKing_C" "Black"))
      (bind _returnvalue_3 (`|SpawnActorFromClass` "/Game/Blueprints/AI/GridsSteps/King/BP_GridStepsKing.BP_GridStepsKing_C" (`KismetMathLibrary.MakeTransform` (`self.K2_GetActorLocation` (`|GetArrayItem` (`self.GetOverlappingActors` (`|GetArrayItem` _outactors) "/Game/Blueprints/BattleField/BP_Cell.BP_Cell_C")))) "Undefined" "OverrideRootScale" null null))
      (set `local.LGridEnemyKing` _returnvalue_3)
      (else
        (bind _outactors_2 (`GameplayStatics.GetAllActorsOfClassWithTag` "BP_AIChessFigureKing_C" "White"))
        (bind _returnvalue_4 (`|SpawnActorFromClass` "/Game/Blueprints/AI/GridsSteps/King/BP_GridStepsKing.BP_GridStepsKing_C" (`KismetMathLibrary.MakeTransform` (`self.K2_GetActorLocation` (`|GetArrayItem` (`self.GetOverlappingActors` (`|GetArrayItem` _outactors_2) "/Game/Blueprints/BattleField/BP_Cell.BP_Cell_C")))) "Undefined" "OverrideRootScale" null null))
        (set `local.LGridEnemyKing` _returnvalue_4)))
    (for (_array_element _array_index) (`self.K2_GetComponentsByClass` (`local.LGridSelfKing`) "/Script/Engine.BoxComponent")
      (set `local.LBox` _array_element)
      (set `local.LIndex` _array_index)
      (`/Engine/EditorBlueprintResources/StandardMacros.IsValid` (`|GetArrayItem` (`PrimitiveComponent.GetOverlappingActors` (`local.LBox`) "/Game/Blueprints/AI/GridsSteps/King/BP_GridStepsKing.BP_GridStepsKing_C"))
        (:`Is Valid`
          (`self.AttachBox CollisionToDestroyer` (`local.LBox`) (`local.LDestroyerComponents`)))
        (:`Is Not Valid`
          (bind (_ldelleftcastlingboxout_ _ldelrightcastlingboxout_) (`self.HandlerAvailableStepsKing` (`local.LBox`) (`local.LDestroyerComponents`)))
          (if _ldelleftcastlingboxout_
            (set `local.LDelLeftCastlingBox?` true))
          (if _ldelrightcastlingboxout_
            (set `local.LDelRightCastlingBox?` true)))))
    (if (== (`self.GridType`) "/Game/Blueprints/AI/GridsSteps/King/BP_GridStepsKing.BP_GridStepsKing_C")
      (`self.K2_DestroyActor` (`local.LGridSelfKing`))
      (`self.K2_DestroyActor` (`local.LGridEnemyKing`))
      (`self.K2_DestroyActor` (`local.LDestroyerComponents`))
      (else
        (bind _outactors_3 (`GameplayStatics.GetAllActorsOfClassWithTag` "/Game/Blueprints/AI/ChessFigure/BP_AIChessFigureRook.BP_AIChessFigureRook_C" (`|GetArrayItem` (`self.Tags`))))
        (for _array_element_2 _outactors_3
          (switch `string` (`/Game/Blueprints/AI/ChessFigure/BP_AIChessFigureRook.RookSide` _array_element_2)
            (:`Left`
              (bind _firststepused_ (`/Game/Blueprints/AI/ChessFigure/BP_AIChessFigureBase.FirstStepUsed?` _array_element_2))
              (if _firststepused_
                (set `local.LDelLeftCastlingBox?` true)))
            (:`Right`
              (if _firststepused_
                (set `local.LDelRightCastlingBox?` true)))))
        (for _array_element_3 (`self.K2_GetComponentsByClass` (`local.LGridSelfKing`) "/Script/Engine.BoxComponent")
          (set `local.LBox` _array_element_3)
          (if (not (== (`KismetArrayLibrary.Array_Length` (`ActorComponent.ComponentTags` (`local.LBox`))) 0))
            (switch `name` (`|GetArrayItem` (`ActorComponent.ComponentTags` (`local.LBox`)))
              (:`LeftCastling`
                (if (`local.LDelLeftCastlingBox?`)
                  (`self.AttachBox CollisionToDestroyer` (`local.LBox`) (`local.LDestroyerComponents`) :!label _label)
                  (elif (`KismetArrayLibrary.Array_IsValidIndex` (`ActorComponent.ComponentTags` (`local.LBox`)) 1)
                    (`self.AttachBox CollisionToDestroyer` (`local.LBox`) (`local.LDestroyerComponents`))
                    (else
                      (`self.ShowAvailableStep` (`local.LBox`))))))
              (:`RightCastling`
                (if (`local.LDelRightCastlingBox?`)
                  (goto _label)
                  (else
                    (`self.ShowAvailableStep` (`local.LBox`))))))))
        (`self.K2_DestroyActor` (`local.LGridSelfKing`))
        (`self.K2_DestroyActor` (`local.LGridEnemyKing`))
        (`self.K2_DestroyActor` (`local.LDestroyerComponents`))))))

(fn `UserConstructionScript`
  (`parent.UserConstructionScript`))