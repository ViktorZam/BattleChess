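; AI chess rook Blueprint that computes straight-line moves and takes part in check evaluation.
; On BeginPlay it reads its overlapped cell's tag to set RookSide, which is "Left" for all four corners, and it records its first step once.
; The check event runs CalculateStepsRook, scanning four directions to the board edge via cell-name strings, filling AvailableMoves and calling helpers to disable figures and check threat-removing cells.
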(event `self.ReceiveBeginPlay`
  (bind _output (`|GetArrayItem` (`self.GetOverlappingActors` "/Game/Blueprints/BattleField/BP_Cell.BP_Cell_C")))
  (`parent.ReceiveBeginPlay`)
  (`/Engine/EditorBlueprintResources/StandardMacros.IsValid` _output
    (:`Is Valid`
      (switch `name` (`|GetArrayItem` (`Actor.Tags` _output))
        (:`a1`
          (set `self.RookSide` "Left" :!label _label))
        (:`a8`
          (goto _label))
        (:`h1`
          (set `self.RookSide` "Left" :!label _label_2))
        (:`h8`
          (goto _label_2))))))

(event `/Game/Blueprints/Interfaces/BPI_Figures.SetUsedFirstStep`
  (`/Engine/EditorBlueprintResources/StandardMacros.DoOnce` false
    (:`Completed`
      (set `self.FirstStepUsed?` true))))

(event `/Game/Blueprints/Interfaces/BPI_Figures.CalculateCheck/DisableFigures`
  (params (Attacker :type "/Game/Blueprints/AI/ChessFigure/BP_AIChessFigureBase Object Reference") (CellsOfAttacker :type "Array of Name (by ref)") (CellsRemoveThreat :type "Array of String (by ref)"))
  (`self.CalculateStepsRook` Attacker CellsOfAttacker CellsRemoveThreat))

(fn `CalculateStepsRook`
  (params (Attacker :type "/Game/Blueprints/AI/ChessFigure/BP_AIChessFigureBase Object Reference") (CellsOfAttacker :type "Array of Name (by ref)") (CellsRemoveThreat :type "Array of String (by ref)"))
  (locals (LPositionCell :type Name) (LDisableFigure :type "Array of /Game/Blueprints/AI/ChessFigure/BP_AIChessFigureBase Object Reference") (LDifferenceSignAndNumberInPosition :type Integer))
  (set `local.LPositionCell` (`|GetArrayItem` (`Actor.Tags` (`|GetArrayItem` (`self.GetOverlappingActors` "/Game/Blueprints/BattleField/BP_Cell.BP_Cell_C")))))
  (for _index (range 8)
    (switch `int` _index
      (:`0`
        ;[1 1 1] Up
        (for _index_2 (range (`KismetStringLibrary.Conv_StringToInt` (`KismetStringLibrary.GetSubstring` (`KismetStringLibrary.Conv_NameToString` (`local.LPositionCell`)) 1)) 9)
          (bind _returnvalue (`KismetStringLibrary.Conv_StringToName` (`KismetStringLibrary.Concat_StrStr` (`KismetStringLibrary.GetSubstring` (`KismetStringLibrary.Conv_NameToString` (`local.LPositionCell`))) (`KismetStringLibrary.Conv_IntToString` _index_2))))
          (`KismetArrayLibrary.Array_AddUnique` (`self.AvailableMoves`) _returnvalue)
          (`self.CalculateCheck/FindFigureForDisable` _returnvalue (`local.LPositionCell`) (`local.LDisableFigure`) true (`local.Attacker`) (`local.CellsOfAttacker`) (`local.CellsRemoveThreat`)))
        (`self.DisableFigure` (`local.LDisableFigure`))
        (`self.Check Cells Remove Threat` (`local.Attacker`) (`local.CellsRemoveThreat`)))
      (:`1`
        ;[1 1 1] Right
        (for _index_3 (range (`KismetArrayLibrary.Array_Find` (`|MakeArray` "a" "b" "c" "d" "e" "f" "g" "h") (`KismetStringLibrary.GetSubstring` (`KismetStringLibrary.Conv_NameToString` (`local.LPositionCell`)))) 8)
          (bind _returnvalue_2 (`KismetStringLibrary.Conv_StringToName` (`KismetStringLibrary.Concat_StrStr` (`|GetArrayItem` (`|MakeArray` "a" "b" "c" "d" "e" "f" "g" "h") _index_3) (`KismetStringLibrary.GetSubstring` (`KismetStringLibrary.Conv_NameToString` (`local.LPositionCell`)) 1))))
          (`KismetArrayLibrary.Array_AddUnique` (`self.AvailableMoves`) _returnvalue_2)
          (`self.CalculateCheck/FindFigureForDisable` _returnvalue_2 (`local.LPositionCell`) (`local.LDisableFigure`) true (`local.Attacker`) (`local.CellsOfAttacker`) (`local.CellsRemoveThreat`)))
        (`self.DisableFigure` (`local.LDisableFigure`))
        (`self.Check Cells Remove Threat` (`local.Attacker`) (`local.CellsRemoveThreat`)))
      (:`2`
        ;[1 1 1] Down
        (for _index_4 (range (* (`KismetStringLibrary.Conv_StringToInt` (`KismetStringLibrary.GetSubstring` (`KismetStringLibrary.Conv_NameToString` (`local.LPositionCell`)) 1)) -1) 0)
          (bind _returnvalue_3 (`KismetStringLibrary.Conv_StringToName` (`KismetStringLibrary.Concat_StrStr` (`KismetStringLibrary.GetSubstring` (`KismetStringLibrary.Conv_NameToString` (`local.LPositionCell`))) (`KismetStringLibrary.Conv_IntToString` (* _index_4 -1)))))
          (`KismetArrayLibrary.Array_AddUnique` (`self.AvailableMoves`) _returnvalue_3)
          (`self.CalculateCheck/FindFigureForDisable` _returnvalue_3 (`local.LPositionCell`) (`local.LDisableFigure`) true (`local.Attacker`) (`local.CellsOfAttacker`) (`local.CellsRemoveThreat`)))
        (`self.DisableFigure` (`local.LDisableFigure`))
        (`self.Check Cells Remove Threat` (`local.Attacker`) (`local.CellsRemoveThreat`)))
      (:`3`
        ;[1 1 1] Left
        (for _index_5 (range (`KismetArrayLibrary.Array_Find` (`|MakeArray` "h" "g" "f" "e" "d" "c" "b" "a") (`KismetStringLibrary.GetSubstring` (`KismetStringLibrary.Conv_NameToString` (`local.LPositionCell`)))) 8)
          (bind _returnvalue_4 (`KismetStringLibrary.Conv_StringToName` (`KismetStringLibrary.Concat_StrStr` (`|GetArrayItem` (`|MakeArray` "h" "g" "f" "e" "d" "c" "b" "a") _index_5) (`KismetStringLibrary.GetSubstring` (`KismetStringLibrary.Conv_NameToString` (`local.LPositionCell`)) 1))))
          (`KismetArrayLibrary.Array_AddUnique` (`self.AvailableMoves`) _returnvalue_4)
          (`self.CalculateCheck/FindFigureForDisable` _returnvalue_4 (`local.LPositionCell`) (`local.LDisableFigure`) true (`local.Attacker`) (`local.CellsOfAttacker`) (`local.CellsRemoveThreat`)))
        (`self.DisableFigure` (`local.LDisableFigure`))
        (`self.Check Cells Remove Threat` (`local.Attacker`) (`local.CellsRemoveThreat`))))))

(fn `UserConstructionScript`
  (`parent.UserConstructionScript`))