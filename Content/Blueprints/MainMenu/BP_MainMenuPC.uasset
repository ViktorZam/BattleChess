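; Main menu player controller that hides the cursor on start, destroys any existing session and holds back UI control until Steam is detected.
; A looping one-second timer polls for the Steam online subsystem.
; When Steam is found, or once game time passes five seconds, it stops polling and enables the cursor with UI-only input focused on the HUD's main menu widget.
; On timeout it also shows the HUD's no-Steam widget.
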(event `self.ReceiveBeginPlay`
  (set `self.bShowMouseCursor` false)
  (bind _returnvalue (`KismetSystemLibrary.K2_SetTimerDelegate` (delegate `CheckSteam`) 1.0 true))
  (set `self.LoadSteam` _returnvalue)
  (`DestroySessionCallbackProxy.DestroySession` self))

(event `CheckSteam`
  (if (`AdvancedSessionsLibrary.HasOnlineSubsystem` "steam")
    (`self.EnableControl`)
    (`KismetSystemLibrary.K2_ClearAndInvalidateTimerHandle` (`self.LoadSteam`))
    (elif (> (`KismetSystemLibrary.GetGameTimeInSeconds`) 5.0)
      (`UserWidget.AddToViewport` (`/Game/Blueprints/MainMenu/BP_MainMenuHUD.NoSteamWidget` (cast `/Game/Blueprints/MainMenu/BP_MainMenuHUD` (`self.GetHUD`) :!pure true)) 0)
      (`self.EnableControl`)
      (`KismetSystemLibrary.K2_ClearAndInvalidateTimerHandle` (`self.LoadSteam`)))))

(event `EnableControl`
  (set `self.bShowMouseCursor` true)
  (`WidgetBlueprintLibrary.SetInputMode_UIOnlyEx` self (`/Game/Blueprints/MainMenu/BP_MainMenuHUD.MainMenuWidget` (cast `/Game/Blueprints/MainMenu/BP_MainMenuHUD` (`self.GetHUD` self) :!pure true))))

(fn `UserConstructionScript`)