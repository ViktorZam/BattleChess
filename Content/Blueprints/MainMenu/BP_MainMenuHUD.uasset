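; Main menu HUD that sets up the front-end UI widgets when play begins.
; It creates the main menu, online game menu, lobby creation, find game and no-Steam widgets, storing each in a variable.
; Only the main menu is added to the viewport; the others are pre-created but not displayed by this Blueprint.
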(event `self.ReceiveBeginPlay`
  (bind _returnvalue (`|CreateWidget` "/Game/Widgets/MainMenu/WBP_MainMenu.WBP_MainMenu_C"))
  (bind _output_get (set `self.MainMenuWidget` _returnvalue))
  (`UserWidget.AddToViewport` _output_get 0)
  (bind _returnvalue_2 (`|CreateWidget` "/Game/Widgets/MainMenu/WBP_OnlineGameMenu.WBP_OnlineGameMenu_C"))
  (set `self.OnlineGameMenuWidget` _returnvalue_2)
  (bind _returnvalue_3 (`|CreateWidget` "/Game/Widgets/LobbyOnlineGame/WBP_LobbyCreateOnlineGame.WBP_LobbyCreateOnlineGame_C"))
  (set `self.LobbyCreateOnlineGameWidget` _returnvalue_3)
  (bind _returnvalue_4 (`|CreateWidget` "/Game/Widgets/MainMenu/WBP_FindOnlineGame.WBP_FindOnlineGame_C"))
  (set `self.FindOnlineGameWidget` _returnvalue_4)
  (bind _returnvalue_5 (`|CreateWidget` "/Game/Widgets/MainMenu/WBP_NoSteam.WBP_NoSteam_C"))
  (set `self.NoSteamWidget` _returnvalue_5))

(fn `UserConstructionScript`)